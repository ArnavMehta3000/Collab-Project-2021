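; BP_TestPlayer is a first-person-style test player character with movement, shooting, magnet grenades, a shield and a slow-time toggle.
; Firing and reloading go through ShootingComponent, which receives muzzle location and actor rotation each tick once the first shot opens a gate.
; GrenadeComponent throws along camera rotation, and ArnavGameMode handles time changes.
; BeginPlay spawns and attaches a BP_PlayerMultiShield, shown while Shield input is held.
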(event `InputAxis|MoveForward`
  (params (AxisValue :type "Float (single-precision)"))
  ;[1 1 1] Movement
  (`self.AddMovementInput` (`self.GetActorForwardVector`) AxisValue))

(event `InputAxis|Turn`
  (params (AxisValue :type "Float (single-precision)"))
  ;[1 1 1] Look
  (`self.AddControllerYawInput` AxisValue))

(event `InputAxis|LookUp`
  (params (AxisValue :type "Float (single-precision)"))
  ;[1 1 1] Look
  (`self.AddControllerPitchInput` (* (`self.GetInputAxisKeyValue`) -1.0)))

(event `InputAxis|MoveRight`
  (params (AxisValue :type "Float (single-precision)"))
  ;[1 1 1] Movement
  (`self.AddMovementInput` (`self.GetActorRightVector`) AxisValue))

(event `InputAction|Jump`
  (params (Key :type "Key Structure"))
  ;[1 1 1] Jumping
  (:`Pressed`
    (if (`NavMovementComponent.IsMovingOnGround` (`self.CharacterMovement`))
      (`self.Jump`))))

(event `self.ReceiveTick`
  (params (DeltaSeconds :type "Float (single-precision)"))
  ;[1 1 1] Shooting
  (`/Engine/EditorBlueprintResources/StandardMacros.Gate` true :!label _label
    (:`Exit`
      (`/Game/Arnav/Shooting/ShootingComponent.UpdateVariables` (`self.ShootingComponent`) (`SceneComponent.K2_GetComponentLocation` (`self.Muzzle`)) (`self.K2_GetActorRotation`) null))))

(event `InputAction|Fire`
  (params (Key :type "Key Structure"))
  (bind _shootingcomponent (`self.ShootingComponent`))
  ;[1 1 1] Shooting
  (:`Pressed`
    (`/Game/Arnav/Shooting/ShootingComponent.Fire Weapon` _shootingcomponent true (`SceneComponent.K2_GetComponentLocation` (`self.Muzzle`)) (`self.K2_GetActorRotation`))
    (goto _label :!via `Open`))
  (:`Released`
    (`/Game/Arnav/Shooting/ShootingComponent.FIre Release` _shootingcomponent)))

(event `Key|One`
  (params (Key :type "Key Structure"))
  (bind _asarnav_game_mode (cast `/Game/Arnav/ArnavGameMode` (`GameplayStatics.GetGameMode`) :!pure true))
  (:`Pressed`
    (`/Engine/EditorBlueprintResources/StandardMacros.FlipFlop`
      (:`A`
        (`/Game/Arnav/ArnavGameMode.Slow Time` _asarnav_game_mode))
      (:`B`
        (`/Game/Arnav/ArnavGameMode.Normal TIme` _asarnav_game_mode)))))

(event `Key|G`
  (params (Key :type "Key Structure"))
  ;[1 1 1] Grenades Stuff
  (:`Pressed`
    (`/Game/Arnav/Grenades/GrenadeComponent.ThrowGrenade` (`self.GrenadeComponent`) "/Game/Arnav/Grenades/GrenadeTypes/BP_MagnetGrenade.BP_MagnetGrenade_C" (`SceneComponent.K2_GetComponentLocation` (`self.Muzzle`)) (`SceneComponent.K2_GetComponentRotation` (`self.Camera`)) 0.1 (`self.grenadeThrowForce`))))

(event `self.ReceiveBeginPlay`
  (`self.Setup Shield`))

(event `Key|R`
  (params (Key :type "Key Structure"))
  (:`Pressed`
    (`/Game/Arnav/Shooting/ShootingComponent.Reload` (`self.ShootingComponent`))))

(event `Setup Shield`
  (bind _shield_hold_point (`self.Shield Hold Point`))
  ;[1 1 1] Give player shield, attach it and then hide it
  (bind _returnvalue (`|SpawnActorFromClass` "/Game/Arnav/Shield/BP_PlayerMultiShield.BP_PlayerMultiShield_C" (`SceneComponent.K2_GetComponentToWorld` _shield_hold_point) "Undefined" "OverrideRootScale" null null)) ; Set type of shield here
  (`self.K2_AttachToComponent` _returnvalue _shield_hold_point "None" "KeepWorld" "KeepWorld" "KeepWorld" false)
  (bind _output_get (set `self.playerShield` _returnvalue))
  (`/Game/Arnav/Shield/BP_PlayerShieldBase.Initialize` _output_get 1.0 5.0 3.0 false false))

(event `InputAction|Shield`
  (params (Key :type "Key Structure"))
  (:`Pressed`
    (`self.ShowShield`))
  (:`Released`
    (`self.Hide Shield`)))

(event `ShowShield`
  (set `self.isShieldActive` true)
  (`/Game/Arnav/Shield/BP_PlayerShieldBase.Show` (`self.playerShield`)))

(event `Hide Shield`
  (set `self.isShieldActive` false)
  (`/Game/Arnav/Shield/BP_PlayerShieldBase.Hide` (`self.playerShield`)))

(fn `UserConstructionScript`)