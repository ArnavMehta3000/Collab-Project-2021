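; BP_Bullet is a bouncing projectile actor that delivers damage, credited to its owner, through a hit-message interface.
; InitializeBullet stores owner, damage and bounce limit, then sets local forward velocity and activates the ProjectileMovement component.
; Overlaps (ignoring other bullets) and hits send IHitMessage and destroy the bullet when it returns true; exhausting bounces also destroys it.
; An interface getter exposes the movement component with Reflect false; other getters are empty.
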(event `self.ProjectileMovement.OnProjectileBounce`
  (params (ImpactResult :type "HitResult Structure (by ref)") (ImpactVelocity :type "Vector Structure (by ref)"))
  (bind _result (`/Engine/EditorBlueprintResources/StandardMacros.DecrementInt` (`self.currentBounce`))
    (:`  `
      (if (<= _result 0)
        (`self.K2_DestroyActor`)))))

(event `self.ReceiveActorBeginOverlap`
  (params (OtherActor :type "Actor Object Reference"))
  (if (not (== (`GameplayStatics.GetObjectClass` OtherActor) "BP_Bullet_C"))
    (bind _succsess (message `/Game/Rowan/I_Hit.I_Hit` OtherActor (`self.player`) (`self.damage`)))
    (if _succsess
      (`self.K2_DestroyActor`))))

(event `self.ReceiveHit`
  (params (MyComp :type "PrimitiveComponent Object Reference") (Other :type "Actor Object Reference") (OtherComp :type "PrimitiveComponent Object Reference") (bSelfMoved :type Boolean) (HitLocation :type "Vector Structure") (HitNormal :type "Vector Structure") (NormalImpulse :type "Vector Structure") (Hit :type "HitResult Structure (by ref)"))
  (bind _succsess (message `/Game/Rowan/I_Hit.I_Hit` Other (`self.player`) (`self.damage`)))
  (if _succsess
    (`self.K2_DestroyActor`)))

(fn `I_Get Player Character`
  (returns (NewParam :type "/Game/Rowan/FirstPersonCharacterROwan Object Reference"))
  (return null))

(fn `I_GetGameMode`
  (returns (GetGameMode :type "/Game/Skye/FirstPersonTemplateBlueprints(TheseHaveBeenEdits)/FirstPersonGameModeSKYE Object Reference"))
  (return null))

(fn `I_GetPortaTurret`
  (returns (`Porta Turret` :type "/Game/Rowan/Porta_turret Object Reference"))
  (return null))

(fn `I_GetProjectileMovement`
  (returns (NewParam :type "ProjectileMovementComponent Object Reference") (Reflect :type Boolean))
  (return (`self.ProjectileMovement`) false))

(fn `InitializeBullet`
  (params (owner :type "Actor Object Reference") (bulletSpeed :type "Float (double-precision)") (damageAmount :type "Float (double-precision)") (bounceCount :type Integer))
  (bind _projectilemovement (`self.ProjectileMovement`))
  (set `self.player` owner)
  (`ProjectileMovementComponent.SetVelocityInLocalSpace` _projectilemovement (`KismetMathLibrary.MakeVector` bulletSpeed))
  (set `self.damage` damageAmount)
  (bind _output_get (set `self.maxBounce` (+ bounceCount 1)))
  (set `self.currentBounce` _output_get)
  (`ActorComponent.Activate` _projectilemovement false))

(fn `UserConstructionScript`)