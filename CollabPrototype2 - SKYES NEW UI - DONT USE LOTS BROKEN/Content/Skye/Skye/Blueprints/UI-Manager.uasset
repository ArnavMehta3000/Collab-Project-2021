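; UI manager for the in-game HUD, acting as a single facade between gameplay code and the InGameUI child widgets.
; Init creates and adds InGameUI for the Game World case, then seeds health, portrait, build points, four abilities, ultimate, ammo and combo text.
; Separate pass-through events forward later updates, such as ability uses and recharge, ult charge and ammo changes, straight to the matching sub-widget.
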(event `Init`
  (params (CurrentWorld :type "/Game/PT1/SkyeUI/Content/Skye/Enums/E_World Enum" :default "NewEnumerator0") (`Current Player Health` :type "Float (double-precision)") (`Max Player Health` :type "Float (double-precision)") (`Player PFP` :type "Object Object Reference") (`Current Build Points` :type Text) (`AB1 Max Number of Ability Uses BASE` :type Integer) (`AB1 TimeToRegen` :type "Float (double-precision)") (`AB1 Key` :type Text) (`AB2 Max Number of Ability Uses BASE` :type Integer) (`AB2 TimeToRegen` :type "Float (double-precision)") (`AB2 Key` :type Text) (`AB3 Max Number of Ability Uses BASE` :type Integer) (`AB3 TimeToRegen` :type "Float (double-precision)") (`AB3 Key` :type Text) (`AB4 Max Number of Ability Uses BASE` :type Integer) (`AB4 TimeToRegen` :type "Float (double-precision)") (`AB4 Key` :type Text) (UltChargeValue :type "Float (double-precision)") (MaxUltChargeValue :type "Float (double-precision)") (`Ultimate Image Background` :type "Object Object Reference") (`Ult Key` :type Text) (CurrentAmmoAmount :type Integer) (CurrentRemainingClips :type Integer) (AmmoPerClip :type Integer) (`Combo Text` :type Text))
  (`|ExecutionSequence`
    (:`then_0`
      (switch `/Game/PT1/SkyeUI/Content/Skye/Enums/E_World` CurrentWorld
        (:`NewEnumerator1`
          (bind _returnvalue (`|CreateWidget` "/Game/Skye/Skye/UI/InGameUI.InGameUI_C"))
          (bind _output_get (set `self.InGameUI` _returnvalue))
          (`UserWidget.AddToViewport` _output_get 0))))
    (:`then_1`
      (`self.Update Player Health Bar` `Current Player Health` `Max Player Health`)
      (`self.Update Player PFP` `Player PFP`))
    (:`then_2`
      (`self.Update Build Text` `Current Build Points`))
    (:`then_3`
      (`self.AB1 Init` `AB1 Max Number of Ability Uses BASE` `AB1 TimeToRegen` `AB1 Key`))
    (:`then_4`
      (`self.AB2 Init` `AB2 Max Number of Ability Uses BASE` `AB2 TimeToRegen` `AB2 Key`))
    (:`then_5`
      (`self.AB3 Init` `AB3 Max Number of Ability Uses BASE` `AB3 TimeToRegen` `AB3 Key`))
    (:`then_6`
      (`self.AB4 Init` `AB4 Max Number of Ability Uses BASE` `AB4 TimeToRegen` `AB4 Key`))
    (:`then_7`
      (`self.Ult Init` UltChargeValue MaxUltChargeValue `Ultimate Image Background` `Ult Key`))
    (:`then_8`
      (`self.Ammo Init` CurrentAmmoAmount CurrentRemainingClips AmmoPerClip))
    (:`then_9`
      (`self.Update Combo Text` `Combo Text`))))

(event `Update Combo Text`
  (params (`Combo Text` :type Text))
  ;[1 1 1] Combo
  (`/Game/Skye/Skye/UI/Widgets/ComboWidget.UpdateComboText` (`/Game/Skye/Skye/UI/InGameUI.ComboWidget` (`self.InGameUI`)) `Combo Text`))

(event `Update Player Health Bar`
  (params (`Current Health` :type "Float (double-precision)") (`Max Health` :type "Float (double-precision)"))
  ;[1 1 1] Player
  (`/Game/Skye/Skye/UI/Widgets/PlayerStatsWidget.UpdateHealthBar` (`/Game/Skye/Skye/UI/InGameUI.PlayerStatsWidget` (`self.InGameUI`)) `Current Health` `Max Health`))

(event `Update Player PFP`
  (params (Image :type "Object Object Reference"))
  ;[1 1 1] Player
  (`/Game/Skye/Skye/UI/Widgets/PlayerStatsWidget.UpdatePlayerPFP` (`/Game/Skye/Skye/UI/InGameUI.PlayerStatsWidget` (`self.InGameUI`)) Image))

(event `Update Build Text`
  (params (`Current Build Points` :type Text))
  ;[1 1 1] Build Points
  (`/Game/Skye/Skye/UI/Widgets/BuildPointsWidget.UpdateBuildText` (`/Game/Skye/Skye/UI/Widgets/PlayerStatsWidget.BuildPointsWidget` (`/Game/Skye/Skye/UI/InGameUI.PlayerStatsWidget` (`self.InGameUI`))) `Current Build Points`))

(event `AB3 Init`
  (params (`Max Number of Ability Uses BASE` :type Integer) (TimeToRegen :type "Float (double-precision)") (Key :type Text))
  ;[1 1 1] Ability 3
  (`/Game/Skye/Skye/UI/Widgets/AbilityWidget.Init` (`/Game/Skye/Skye/UI/Widgets/AbilityBarWidget.Ability3` (`/Game/Skye/Skye/UI/InGameUI.AbilityBarWidget` (`self.InGameUI`))) `Max Number of Ability Uses BASE` TimeToRegen Key))

(event `AB1 Init`
  (params (`Max Number of Ability Uses BASE` :type Integer) (TimeToRegen :type "Float (double-precision)") (Key :type Text))
  ;[1 1 1] Ability 1
  (`/Game/Skye/Skye/UI/Widgets/AbilityWidget.Init` (`/Game/Skye/Skye/UI/Widgets/AbilityBarWidget.Ability1` (`/Game/Skye/Skye/UI/InGameUI.AbilityBarWidget` (`self.InGameUI`))) `Max Number of Ability Uses BASE` TimeToRegen Key))

(event `AB3 Ability Used`
  ;[1 1 1] Ability 3
  (`/Game/Skye/Skye/UI/Widgets/AbilityWidget.AbilityUsed` (`/Game/Skye/Skye/UI/Widgets/AbilityBarWidget.Ability3` (`/Game/Skye/Skye/UI/InGameUI.AbilityBarWidget` (`self.InGameUI`)))))

(event `AB3 Ability Regened`
  ;[1 1 1] Ability 3
  (`/Game/Skye/Skye/UI/Widgets/AbilityWidget.AbilityRegened` (`/Game/Skye/Skye/UI/Widgets/AbilityBarWidget.Ability3` (`/Game/Skye/Skye/UI/InGameUI.AbilityBarWidget` (`self.InGameUI`)))))

(event `AB1 Ability Used`
  ;[1 1 1] Ability 1
  (`/Game/Skye/Skye/UI/Widgets/AbilityWidget.AbilityUsed` (`/Game/Skye/Skye/UI/Widgets/AbilityBarWidget.Ability1` (`/Game/Skye/Skye/UI/InGameUI.AbilityBarWidget` (`self.InGameUI`)))))

(event `AB3 Update Recharge Bar`
  (params (`Current Value` :type "Float (double-precision)") (`Max Value` :type "Float (double-precision)"))
  ;[1 1 1] Ability 3
  (`/Game/Skye/Skye/UI/Widgets/AbilityWidget.Update Recharge Bar` (`/Game/Skye/Skye/UI/Widgets/AbilityBarWidget.Ability3` (`/Game/Skye/Skye/UI/InGameUI.AbilityBarWidget` (`self.InGameUI`))) `Current Value` `Max Value`))

(event `AB1 Ability Regened`
  ;[1 1 1] Ability 1
  (`/Game/Skye/Skye/UI/Widgets/AbilityWidget.AbilityRegened` (`/Game/Skye/Skye/UI/Widgets/AbilityBarWidget.Ability1` (`/Game/Skye/Skye/UI/InGameUI.AbilityBarWidget` (`self.InGameUI`)))))

(event `AB1 Update Recharge Bar`
  (params (`Current Value` :type "Float (double-precision)") (`Max Value` :type "Float (double-precision)"))
  ;[1 1 1] Ability 1
  (`/Game/Skye/Skye/UI/Widgets/AbilityWidget.Update Recharge Bar` (`/Game/Skye/Skye/UI/Widgets/AbilityBarWidget.Ability1` (`/Game/Skye/Skye/UI/InGameUI.AbilityBarWidget` (`self.InGameUI`))) `Current Value` `Max Value`))

(event `AB3 Update Uses`
  (params (`Current Number of Ability Uses` :type Integer))
  ;[1 1 1] Ability 3
  (`/Game/Skye/Skye/UI/Widgets/AbilityWidget.Update Uses UI` (`/Game/Skye/Skye/UI/Widgets/AbilityBarWidget.Ability3` (`/Game/Skye/Skye/UI/InGameUI.AbilityBarWidget` (`self.InGameUI`))) `Current Number of Ability Uses`))

(event `AB1 Update Uses`
  (params (`Current Number of Ability Uses` :type Integer))
  ;[1 1 1] Ability 1
  (`/Game/Skye/Skye/UI/Widgets/AbilityWidget.Update Uses UI` (`/Game/Skye/Skye/UI/Widgets/AbilityBarWidget.Ability1` (`/Game/Skye/Skye/UI/InGameUI.AbilityBarWidget` (`self.InGameUI`))) `Current Number of Ability Uses`))

(event `AB2 Init`
  (params (`Max Number of Ability Uses BASE` :type Integer) (TimeToRegen :type "Float (double-precision)") (Key :type Text))
  ;[1 1 1] Ability 2
  (`/Game/Skye/Skye/UI/Widgets/AbilityWidget.Init` (`/Game/Skye/Skye/UI/Widgets/AbilityBarWidget.Ability2` (`/Game/Skye/Skye/UI/InGameUI.AbilityBarWidget` (`self.InGameUI`))) `Max Number of Ability Uses BASE` TimeToRegen Key))

(event `AB4 Init`
  (params (`Max Number of Ability Uses BASE` :type Integer) (TimeToRegen :type "Float (double-precision)") (Key :type Text))
  ;[1 1 1] Ability 4
  (`/Game/Skye/Skye/UI/Widgets/AbilityWidget.Init` (`/Game/Skye/Skye/UI/Widgets/AbilityBarWidget.Ability4` (`/Game/Skye/Skye/UI/InGameUI.AbilityBarWidget` (`self.InGameUI`))) `Max Number of Ability Uses BASE` TimeToRegen Key))

(event `AB2 Ability Used`
  ;[1 1 1] Ability 2
  (`/Game/Skye/Skye/UI/Widgets/AbilityWidget.AbilityUsed` (`/Game/Skye/Skye/UI/Widgets/AbilityBarWidget.Ability2` (`/Game/Skye/Skye/UI/InGameUI.AbilityBarWidget` (`self.InGameUI`)))))

(event `AB4 Ability Used`
  ;[1 1 1] Ability 4
  (`/Game/Skye/Skye/UI/Widgets/AbilityWidget.AbilityUsed` (`/Game/Skye/Skye/UI/Widgets/AbilityBarWidget.Ability4` (`/Game/Skye/Skye/UI/InGameUI.AbilityBarWidget` (`self.InGameUI`)))))

(event `AB2 Ability Regened`
  ;[1 1 1] Ability 2
  (`/Game/Skye/Skye/UI/Widgets/AbilityWidget.AbilityRegened` (`/Game/Skye/Skye/UI/Widgets/AbilityBarWidget.Ability2` (`/Game/Skye/Skye/UI/InGameUI.AbilityBarWidget` (`self.InGameUI`)))))

(event `AB4 Ability Regened`
  ;[1 1 1] Ability 4
  (`/Game/Skye/Skye/UI/Widgets/AbilityWidget.AbilityRegened` (`/Game/Skye/Skye/UI/Widgets/AbilityBarWidget.Ability4` (`/Game/Skye/Skye/UI/InGameUI.AbilityBarWidget` (`self.InGameUI`)))))

(event `AB2 Update Recharge Bar`
  (params (`Current Value` :type "Float (double-precision)") (`Max Value` :type "Float (double-precision)"))
  ;[1 1 1] Ability 2
  (`/Game/Skye/Skye/UI/Widgets/AbilityWidget.Update Recharge Bar` (`/Game/Skye/Skye/UI/Widgets/AbilityBarWidget.Ability2` (`/Game/Skye/Skye/UI/InGameUI.AbilityBarWidget` (`self.InGameUI`))) `Current Value` `Max Value`))

(event `AB4 Update Recharge Bar`
  (params (`Current Value` :type "Float (double-precision)") (`Max Value` :type "Float (double-precision)"))
  ;[1 1 1] Ability 4
  (`/Game/Skye/Skye/UI/Widgets/AbilityWidget.Update Recharge Bar` (`/Game/Skye/Skye/UI/Widgets/AbilityBarWidget.Ability4` (`/Game/Skye/Skye/UI/InGameUI.AbilityBarWidget` (`self.InGameUI`))) `Current Value` `Max Value`))

(event `AB2 Update Uses`
  (params (`Current Number of Ability Uses` :type Integer))
  ;[1 1 1] Ability 2
  (`/Game/Skye/Skye/UI/Widgets/AbilityWidget.Update Uses UI` (`/Game/Skye/Skye/UI/Widgets/AbilityBarWidget.Ability2` (`/Game/Skye/Skye/UI/InGameUI.AbilityBarWidget` (`self.InGameUI`))) `Current Number of Ability Uses`))

(event `AB4 Update Uses`
  (params (`Current Number of Ability Uses` :type Integer))
  ;[1 1 1] Ability 4
  (`/Game/Skye/Skye/UI/Widgets/AbilityWidget.Update Uses UI` (`/Game/Skye/Skye/UI/Widgets/AbilityBarWidget.Ability4` (`/Game/Skye/Skye/UI/InGameUI.AbilityBarWidget` (`self.InGameUI`))) `Current Number of Ability Uses`))

(event `Ult Init`
  (params (ChargeValue :type "Float (double-precision)") (MaxChargeValue :type "Float (double-precision)") (`Ultimate Image Background` :type "Object Object Reference") (Key :type Text))
  ;[1 1 1] Ult
  (`/Game/Skye/Skye/UI/Widgets/UltimateAbilityWidget.Init` (`/Game/Skye/Skye/UI/Widgets/AbilityBarWidget.UltimateAbility` (`/Game/Skye/Skye/UI/InGameUI.AbilityBarWidget` (`self.InGameUI`))) ChargeValue MaxChargeValue `Ultimate Image Background` Key))

(event `Ult Update`
  (params (`Charge Percent` :type "Float (double-precision)") (`Max Charge Percent` :type "Float (double-precision)"))
  ;[1 1 1] Ult
  (`/Game/Skye/Skye/UI/Widgets/UltimateAbilityWidget.Update Ult UI` (`/Game/Skye/Skye/UI/Widgets/AbilityBarWidget.UltimateAbility` (`/Game/Skye/Skye/UI/InGameUI.AbilityBarWidget` (`self.InGameUI`))) `Charge Percent` `Max Charge Percent`))

(event `Ammo Init`
  (params (CurrentAmmoAmount :type Integer) (CurrentRemainingClips :type Integer) (AmmoPerClip :type Integer))
  ;[1 1 1] Ammo
  (`/Game/Skye/Skye/UI/Widgets/AmmoWidget.Init` (`/Game/Skye/Skye/UI/InGameUI.AmmoWidget` (`self.InGameUI`)) CurrentAmmoAmount CurrentRemainingClips AmmoPerClip))

(event `Use Ammo`
  ;[1 1 1] Ammo
  (`/Game/Skye/Skye/UI/Widgets/AmmoWidget.UseAmmoUI` (`/Game/Skye/Skye/UI/InGameUI.AmmoWidget` (`self.InGameUI`))))

(event `Add Ammo`
  (params (AmmoToAdd :type Integer))
  ;[1 1 1] Ammo
  (`/Game/Skye/Skye/UI/Widgets/AmmoWidget.AddAmmoUI` (`/Game/Skye/Skye/UI/InGameUI.AmmoWidget` (`self.InGameUI`)) AmmoToAdd))

(fn `UserConstructionScript`)