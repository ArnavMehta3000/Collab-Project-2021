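; TestDummy is a damageable target actor with a health bar and floating damage numbers.
; It starts at max HP, and each TakeDamage call lowers HP, updates the HPBarUI widget, spawns a damage number and checks for death.
; DamageIndicator actors spawn around a scene point with random Y and Z offsets in world space.
; At zero HP, the dummy destroys any remaining indicators and then itself.
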(event `self.ReceiveBeginPlay`
  (`self.OnSpawn`))

(event `OnSpawn`
  (bind _maxhp (`self.MaxHP`))
  ;[1 1 1] Init
  (set `self.CurrentHP` (`self.MaxHP`))
  (set `self.HPBar UI` (cast `/Game/Skye/UIBlueprints/HPBarUI` (`WidgetComponent.GetUserWidgetObject` (`self.HPBarUI`)) :!pure true))
  (`/Game/Skye/UIBlueprints/HPBarUI.UpdateHPBarUI` (`self.HPBar UI`) _maxhp _maxhp))

(event `TakeDamage`
  (params (Damage :type "Float (double-precision)"))
  (bind _returnvalue (- (`self.CurrentHP`) Damage))
  ;[1 1 1] Take Damage
  (`/Game/Skye/UIBlueprints/HPBarUI.UpdateHPBarUI` (`self.HPBar UI`) _returnvalue (`self.MaxHP`))
  (set `self.CurrentHP` _returnvalue)
  (`|ExecutionSequence`
    (:`then_0`
      (`self.SpawnDamageNumber` (`KismetTextLibrary.Conv_DoubleToText` Damage "HalfToEven")))
    (:`then_1`
      (`self.CheckDeath`))))

(event `CheckDeath`
  ;[1 1 1] CheckDeath
  (if (<= (`self.CurrentHP`) 0.0)
    (for _array_element (`self.DamageIndicators`)
      (if (`KismetSystemLibrary.IsValid` _array_element)
        (`self.K2_DestroyActor` _array_element)))
    (`self.K2_DestroyActor`)))

(fn `SpawnDamageNumber`
  (params (DamageNumber :type Text))
  (bind _possibledamagenumberspawnlocationsaroundcenter (`self.PossibleDamageNumberSpawnLocationsAroundCenter`))
  (bind _returnvalue (`SceneComponent.K2_GetComponentToWorld` (`self.DamageNumberSpawnLocation`)))
  (bind _returnvalue_2 (`|SpawnActorFromClass` "/Game/Skye/Blueprints/DamageIndicator.DamageIndicator_C" (`KismetMathLibrary.MakeTransform` (`KismetMathLibrary.MakeVector` (.x (.location _returnvalue)) (`KismetMathLibrary.RandomFloatInRange` (- (.y (.location _returnvalue)) _possibledamagenumberspawnlocationsaroundcenter) (+ (.y (.location _returnvalue)) _possibledamagenumberspawnlocationsaroundcenter)) (`KismetMathLibrary.RandomFloatInRange` (- (.z (.location _returnvalue)) _possibledamagenumberspawnlocationsaroundcenter) (+ (.z (.location _returnvalue)) _possibledamagenumberspawnlocationsaroundcenter))) (.rotation _returnvalue)) "Undefined" "OverrideRootScale" null null))
  (`/Game/Skye/Blueprints/DamageIndicator.SetDamageNumber` _returnvalue_2 DamageNumber)
  (`KismetArrayLibrary.Array_Add` (`self.DamageIndicators`) _returnvalue_2))

(fn `UserConstructionScript`)