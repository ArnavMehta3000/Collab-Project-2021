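; Grid actor that lays out a cell grid from GridData and visualizes it with debug spheres on BeginPlay.
; InitGrid clears old debug drawing, then loops width along Y and depth along X, offsetting points by half the grid size to center them on world origin.
; A helper converts world positions to grid indices by truncating position over cell size, without applying that centering offset.
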(event `self.ReceiveBeginPlay`
  (`self.Init Grid`))

(event `Init Grid`
  (bind (_griddata_width _griddata_depth _griddata_cellsize) (break `/Game/Arnav/Blueprints/Grid/E_GridData` (`self.gridData`)))
  (bind (_griddata_width_2 _griddata_depth_2 _griddata_cellsize_2) (break `/Game/Arnav/Blueprints/Grid/E_GridData` (`self.gridData`)))
  (bind (_griddata_width_3 _griddata_depth_3 _griddata_cellsize_3 _griddata_heightoffset) (break `/Game/Arnav/Blueprints/Grid/E_GridData` (`self.gridData`)))
  (bind (_halfx _halfy) (`self.GetGridHalfSize` _griddata_width _griddata_depth _griddata_cellsize))
  (`self.Clear Debug`)
  (set `self.halfSizeX` _halfx)
  (set `self.halfSizeY` _halfy)
  (for _index (range _griddata_width_2)
    (for _index_2 (range _griddata_depth_2)
      (`KismetSystemLibrary.DrawDebugSphere` (`KismetMathLibrary.MakeVector` (- (* _index_2 _griddata_cellsize_2) (`self.halfSizeX`)) (- (* _index _griddata_cellsize_2) (`self.halfSizeY`)) _griddata_heightoffset) 50.0 12 (struct :`R` 1.0 :`G` 1.0 :`B` 1.0 :`A` 1.0) 100.0 1.0))))

(event `Clear Debug`
  ;[1 1 1] Clear Debug Info
  (`KismetSystemLibrary.FlushDebugStrings`)
  (`KismetSystemLibrary.FlushPersistentDebugLines`))

(fn `Get Grid Point From World Position`
  (params (position :type "Vector Structure"))
  (returns (X :type Integer) (Y :type Integer))
  (bind (_griddata_width _griddata_depth _griddata_cellsize) (break `/Game/Arnav/Blueprints/Grid/E_GridData` (`self.gridData`)))
  (return (`KismetMathLibrary.FTrunc` (/ position_X _griddata_cellsize)) (`KismetMathLibrary.FTrunc` (/ position_Y _griddata_cellsize))))

(fn `GetGridHalfSize`
  (params (width :type Integer) (depth :type Integer) (cellSize :type "Float (double-precision)"))
  (returns (halfX :type "Float (double-precision)") (halfY :type "Float (double-precision)"))
  (return (/ (* (- depth 1) cellSize) 2.0) (/ (* (- width 1) cellSize) 2.0)))

(fn `UserConstructionScript`)