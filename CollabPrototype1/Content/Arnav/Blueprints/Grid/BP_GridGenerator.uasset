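; Grid generator that builds a 3D lattice of nodes from GridData dimensions and cell sizes on BeginPlay.
; CreateGrid clears old nodes and debug drawing, then fills GridNodes with positions centered on the world origin plus a height offset.
; On completion it draws a fixed-size debug box at each node.
; Helpers convert between world positions and cell indices by cell size alone, ignoring the centering and height offsets.
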(event `self.ReceiveBeginPlay`
  (`self.Create Grid`))

(event `Create Grid`
  (bind ((`CellSizeX_10_A5F16D3D4C238530562362827FCE34F5` _cellsizex) (`CellSizeY_13_960EBD99406AF229654DBF8E92F14ED4` _cellsizey) (`CellSizeZ_22_3F1781A74C430DFDB1EA9EB953018F27` _cellsizez)) (break `/Game/Arnav/Blueprints/Grid/E_GridData` (`self.gridData`)))
  (bind ((`Width_2_2548B3234C7564ED328EE78098FBD3DC` _width) (`Depth_4_0CB769EE4611862D0F2B93BB7C0F031F` _depth) (`Height_19_A8F3F8D840E57D97201210B812D2FCCB` _height)) (break `/Game/Arnav/Blueprints/Grid/E_GridData` (`self.gridData`)))
  (bind ((`Width_2_2548B3234C7564ED328EE78098FBD3DC` _width_2) (`Depth_4_0CB769EE4611862D0F2B93BB7C0F031F` _depth_2) (`Height_19_A8F3F8D840E57D97201210B812D2FCCB` _height_2) (`CellSizeX_10_A5F16D3D4C238530562362827FCE34F5` _cellsizex_2) (`CellSizeY_13_960EBD99406AF229654DBF8E92F14ED4` _cellsizey_2) (`CellSizeZ_22_3F1781A74C430DFDB1EA9EB953018F27` _cellsizez_2)) (break `/Game/Arnav/Blueprints/Grid/E_GridData` (`self.gridData`)))
  (bind (_halfx _halfy _halfz) (`self.GetGridHalfSize` _width_2 _depth_2 _height_2 _cellsizex_2 _cellsizey_2 _cellsizez_2))
  (`self.Clear Debug`)
  (if (<= _height 0)
    (`KismetSystemLibrary.PrintString` "Height cannnot be 0" true true (struct :`R` 1.0 :`A` 1.0) 10.0)
    (else
      (for _index (range _width)
        (for _index_2 (range _depth)
          (for _index_3 (range _height)
            (bind _output_get (set `self.pos` (`KismetMathLibrary.MakeVector` (- (* _index_2 _cellsizex) _halfx) (- (* _index _cellsizey) _halfy) (+ (- (* _index_3 _cellsizez) _halfz) (`.HeightOffset_9_0A6C78BF4A830BB88E91A78C6DE4FB7C` (break `/Game/Arnav/Blueprints/Grid/E_GridData` (`self.gridData`)))))))
            (`KismetArrayLibrary.Array_Add` (`self.gridNodes`) (make `/Game/Arnav/Blueprints/Grid/BP_Node` _output_get)))))
      (`self.Grid Completed`))))

(event `Clear Debug`
  ;[1 1 1] Clear Debug Info
  (`KismetSystemLibrary.FlushDebugStrings`)
  (`KismetSystemLibrary.FlushPersistentDebugLines`)
  (`KismetArrayLibrary.Array_Clear` (`self.gridNodes`))
  (set `self.pos` (0.0 0.0 0.0)))

(event `Grid Completed`
  (`self.Draw Debug`))

(event `Draw Debug`
  (for _array_element (`self.gridNodes`)
    (`KismetSystemLibrary.DrawDebugBox` (`.Position_2_F29774BE4D5C89E8A7FA91B1921DC376` (break `/Game/Arnav/Blueprints/Grid/BP_Node` _array_element)) (`KismetMathLibrary.Conv_DoubleToVector` 50.0) (struct :`R` 1.0 :`B` 0.060046 :`A` 1.0) (struct) 60.0 3.0)))

(fn `CellToWorld Pos`
  (params (cell :type "IntVector Structure"))
  (returns (positiom :type "Vector Structure"))
  (bind (_griddata_width _griddata_depth _griddata_height _griddata_cellsizex _griddata_cellsizey _griddata_cellsizez) (break `/Game/Arnav/Blueprints/Grid/E_GridData` (`self.gridData`)))
  (return (`KismetMathLibrary.MakeVector` (* cell_X _griddata_cellsizex) (* cell_Y _griddata_cellsizey) (* cell_Z _griddata_cellsizez))))

(fn `GetGridHalfSize`
  (params (width :type Integer) (depth :type Integer) (Height :type Integer) (cellSizeX :type "Float (double-precision)") (cellSizeY :type "Float (double-precision)") (cellSizeZ :type "Float (double-precision)"))
  (returns (halfX :type "Float (double-precision)") (halfY :type "Float (double-precision)") (halfZ :type "Float (double-precision)"))
  (return (/ (* (- depth 1) cellSizeX) 2.0) (/ (* (- width 1) cellSizeY) 2.0) (/ (* (- Height 1) cellSizeZ) 2.0)))

(fn `UserConstructionScript`)

(fn `WorldPosToCell`
  (params (position :type "Vector Structure"))
  (returns (cell :type "IntVector Structure"))
  (bind (_griddata_width _griddata_depth _griddata_height _griddata_cellsizex _griddata_cellsizey _griddata_cellsizez) (break `/Game/Arnav/Blueprints/Grid/E_GridData` (`self.gridData`)))
  (return (make `IntVector` (`KismetMathLibrary.Clamp` (`KismetMathLibrary.FTrunc` (/ position_X _griddata_cellsizex)) (* -1 _griddata_width) _griddata_width) (`KismetMathLibrary.Clamp` (`KismetMathLibrary.FTrunc` (/ position_Y _griddata_cellsizey)) (* -1 _griddata_depth) _griddata_depth) (`KismetMathLibrary.Clamp` (`KismetMathLibrary.FTrunc` (/ position_Z _griddata_cellsizez)) (* -1 _griddata_height) _griddata_height))))