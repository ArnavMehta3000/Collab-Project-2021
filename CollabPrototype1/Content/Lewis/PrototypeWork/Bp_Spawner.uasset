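; Prototype wave spawner that spawns enemies at its own location and grows the wave size by two each round.
; FWaveStart stores the incoming list of enemy classes and starts a looping timer to spawn them in order.
; Each spawned enemy is passed to the game mode's EnemyCounter; at the wave limit, the timer clears and the count resets.
; FResetWave is a debug hook that overrides the spawned count.
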(event `self.F_WaveStart`
  (params (EnemyIncrease :type "Array of Actor Class Reference (by ref)"))
  ;[1 1 1] Timer For spawning Enemies
  (set `self.Enemy Increase` EnemyIncrease)
  (bind _returnvalue (`KismetSystemLibrary.K2_SetTimerDelegate` (`|CreateDelegate` :!event `Begin Wave`) 1.5 true))
  (set `self.StopTimer` _returnvalue))

(event `Begin Wave`
  ;[1 1 1] Spawning Logic for The Enemies
  (if (!= (`self.SpawnedEnemies`) (`self.SpawnableEnemies`))
    (bind _returnvalue (`|SpawnActorFromClass` (`|GetArrayItem` (`self.Enemy Increase`) (`self.SpawnedEnemies`)) (`KismetMathLibrary.Conv_VectorToTransform` (`self.K2_GetActorLocation`)) "Undefined" "OverrideRootScale" null null))
    (bind _result (`/Engine/EditorBlueprintResources/StandardMacros.IncrementInt` (`self.SpawnedEnemies`))
      (:`  `
        (`KismetSystemLibrary.PrintString` (`KismetStringLibrary.Conv_IntToString` _result))
        (bind _wavegm (message `/Game/Lewis/PrototypeWork/Bpi_Cast.f_GetGameMode` (`GameplayStatics.GetGameMode`)))
        (`/Game/Lewis/PrototypeWork/WaveGameMode.EnemyCounter` _wavegm _returnvalue)))
    (else
      (`KismetSystemLibrary.K2_ClearAndInvalidateTimerHandle` (`self.StopTimer`))
      (set `self.SpawnedEnemies` 0)
      (set `self.SpawnableEnemies` (+ (`self.SpawnableEnemies`) 2)))))

(event `self.F_ResetWave`
  (params (ResetEnemies :type Integer))
  ;[1 1 1] Debug For Setting Spawned Enemies to 0 (When Pressing "U" To Delete Enemys)
  (bind _output_get (set `self.SpawnedEnemies` ResetEnemies))
  (`KismetSystemLibrary.PrintString` (`KismetStringLibrary.Conv_IntToString` _output_get)))

(fn `f_GetGameMode`)

(fn `UserConstructionScript`)