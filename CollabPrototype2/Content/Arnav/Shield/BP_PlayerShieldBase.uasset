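; Base player shield actor that can be shown or hidden, drains while up, recharges while down, and optionally reflects projectiles.
; One timeline drives the charge, playing forward at the depletion rate and reversing at the recharge rate, with auto-hide when depleted.
; Showing requires a completed recharge unless TriggerAnyTime is set.
; In reflecting mode, overlaps and hits negate projectile velocity through an interface, and IHit returns false.
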(event `Initialize`
  (params (depletionRate :type "Float (double-precision)") (rechargeRate :type "Float (double-precision)") (length :type "Float (double-precision)") (triggerAnyTime :type Boolean) (Reflecting :type Boolean))
  (set `self.depletionRate` depletionRate)
  (set `self.rechargeRate` rechargeRate)
  (bind _output_get (set `self.length` length))
  (`TimelineComponent.SetTimelineLength` (`self.Shield Show Time`) _output_get)
  (set `self.triggerAnyTime` triggerAnyTime)
  (set `self.Reflecting` Reflecting)
  (`self.Hide`))

(event `self.ReceiveActorBeginOverlap`
  (params (OtherActor :type "Actor Object Reference"))
  (if (`self.Reflecting`)
    (bind (_newparam _reflect) (message `/Game/Rowan/I_Cast.I_GetProjectileMovement` OtherActor))
    (if _reflect
      (bind (_velocity_x _velocity_y _velocity_z) (`KismetMathLibrary.BreakVector` (`MovementComponent.Velocity` _newparam)))
      (set `MovementComponent.Velocity` (`KismetMathLibrary.MakeVector` (* -1 _velocity_x) (* -1 _velocity_y) (* -1 _velocity_z)) _newparam))))

(event `Hide`
  (bind _staticmesh (`self.StaticMesh`))
  (set `self.isDepleting` false)
  (`ActorComponent.SetActive` _staticmesh false false)
  (`SceneComponent.SetVisibility` _staticmesh false true)
  (`PrimitiveComponent.SetCollisionEnabled` _staticmesh "NoCollision")
  (`TimelineComponent.SetPlayRate` (`self.Shield Show Time`) (`self.rechargeRate`))
  (bind (_direction _charge) (`Timeline|Shield Show Time` :!via `Reverse` :!label _label)
    (:`Update`
      (set `self.currentCharge` _charge))
    (:`Finished`
      (if (`self.isDepleting`)
        (`self.Hide`)
        (set `self.canUse` false)
        (else
          (set `self.canUse` true))))))

(event `self.ReceiveHit`
  (params (MyComp :type "PrimitiveComponent Object Reference") (Other :type "Actor Object Reference") (OtherComp :type "PrimitiveComponent Object Reference") (bSelfMoved :type Boolean) (HitLocation :type "Vector Structure") (HitNormal :type "Vector Structure") (NormalImpulse :type "Vector Structure") (Hit :type "HitResult Structure (by ref)"))
  (if (`self.Reflecting`)
    (bind (_newparam _reflect) (message `/Game/Rowan/I_Cast.I_GetProjectileMovement` Other))
    (if _reflect
      (bind (_velocity_x _velocity_y _velocity_z) (`KismetMathLibrary.BreakVector` (`MovementComponent.Velocity` _newparam)))
      (set `MovementComponent.Velocity` (`KismetMathLibrary.MakeVector` (* -1 _velocity_x) (* -1 _velocity_y) (* -1 _velocity_z)) _newparam))))

(event `Show`
  (bind _staticmesh (`self.StaticMesh`))
  (if (`self.triggerAnyTime`)
    (set `self.isDepleting` true :!label _label_2)
    (`ActorComponent.SetActive` _staticmesh true false)
    (`SceneComponent.SetVisibility` _staticmesh true true)
    (`PrimitiveComponent.SetCollisionEnabled` _staticmesh "QueryAndPhysics")
    (`TimelineComponent.SetPlayRate` (`self.Shield Show Time`) (`self.depletionRate`))
    (goto _label)
    (elif (`self.canUse`)
      (goto _label_2))))

(fn `GetShieldCharge`
  (returns (currentCharge :type "Float (double-precision)"))
  (return (`self.currentCharge`)))

(fn `I_Hit`
  (params (Instiagator :type "Actor Object Reference (by ref)") (Damage :type "Float (double-precision)"))
  (returns (Succsess :type Boolean))
  (return (not (`self.Reflecting`))))

(fn `UserConstructionScript`)