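; BP_PlayerMultiShield is a player shield Blueprint made of two static meshes that are raised and lowered together, extending a parent shield's Show and Hide events.
; Show runs only if TriggerAnyTime or CanUse is set, then starts depletion, enables both meshes' visibility and collision, and calls the parent.
; Hide stops depletion, deactivates and hides both meshes, disables their collision, and calls the parent.
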(event `self.Show`
  (bind _staticmesh1 (`self.StaticMesh1`))
  (bind _staticmesh2 (`self.StaticMesh2`))
  (if (`self.triggerAnyTime`)
    (set `self.isDepleting` true :!label _label)
    (`ActorComponent.SetActive` _staticmesh1 true false)
    (`SceneComponent.SetVisibility` _staticmesh1 true true)
    (`PrimitiveComponent.SetCollisionEnabled` _staticmesh1 "QueryAndPhysics")
    (`ActorComponent.SetActive` _staticmesh2 true false)
    (`SceneComponent.SetVisibility` _staticmesh2 true true)
    (`PrimitiveComponent.SetCollisionEnabled` _staticmesh2 "QueryAndPhysics")
    (`parent.Show`)
    (elif (`self.canUse`)
      (goto _label))))

(event `self.Hide`
  (bind _staticmesh1 (`self.StaticMesh1`))
  (bind _staticmesh2 (`self.StaticMesh2`))
  (set `self.isDepleting` false)
  (`ActorComponent.SetActive` _staticmesh1 false false)
  (`SceneComponent.SetVisibility` _staticmesh1 false true)
  (`PrimitiveComponent.SetCollisionEnabled` _staticmesh1 "NoCollision")
  (`ActorComponent.SetActive` _staticmesh2 false false)
  (`SceneComponent.SetVisibility` _staticmesh2 false true)
  (`PrimitiveComponent.SetCollisionEnabled` _staticmesh2 "NoCollision")
  (`parent.Hide`))

(fn `UserConstructionScript`)