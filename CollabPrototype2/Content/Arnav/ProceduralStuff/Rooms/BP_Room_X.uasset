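; BP_Room_X is a room Blueprint for procedural level generation that provides spawn locations.
; On BeginPlay it flags itself as having spawn points.
; GetAllSpawnPoints returns the world locations of its four SpawnPoint components as an array.
; The construction script only calls its parent, and overlap and tick events are disabled.
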(event `self.ReceiveBeginPlay`
  (set `self.hasSpawnPoint` true))

(fn `GetAllSpawnPoints`
  (returns (spawnPoints :type "Array of Vector Structure"))
  (return (`|MakeArray` (`SceneComponent.K2_GetComponentLocation` (`self.Spawn Point`)) (`SceneComponent.K2_GetComponentLocation` (`self.Spawn Point1`)) (`SceneComponent.K2_GetComponentLocation` (`self.Spawn Point2`)) (`SceneComponent.K2_GetComponentLocation` (`self.Spawn Point3`)))))

(fn `UserConstructionScript`
  (`parent.UserConstructionScript`))