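; Procedural level generator that, after a short startup delay, spawns a starting room at its own transform and grows a chain of random rooms from it.
; Each step picks a random unused spawn point on the latest room, spawns a random room there, then recurses after a delay.
; Used points are tracked with tolerance-based matching; generation stops at the room limit or a room without spawn points.
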(event `self.ReceiveBeginPlay`
  (`KismetSystemLibrary.Delay` 5.0)
  (bind _returnvalue (`|SpawnActorFromClass` "/Game/Arnav/ProceduralStuff/Rooms/BP_Room_X.BP_Room_X_C" (`self.GetTransform`) "Undefined" "OverrideRootScale" null null))
  (`self.Generate` _returnvalue))

(event `Generate`
  (params (room :type "/Game/Arnav/ProceduralStuff/Rooms/BP_RoomBase Object Reference"))
  (`KismetSystemLibrary.PrintString` (`KismetStringLibrary.Concat_StrStr` "Current Count: " (`KismetStringLibrary.Conv_IntToString` (`self.current`))))
  (`self.LimitCheck`
    (:`isInLimit`
      (if (`/Game/Arnav/ProceduralStuff/Rooms/BP_RoomBase.HasSpawnPoints` room)
        (bind _spawnpoints (`/Game/Arnav/ProceduralStuff/Rooms/BP_RoomBase.GetAllSpawnPoints` room :!label _label)) ; Get random spawn point from room
        (bind _output_get (set `self.currentPoint` (`KismetArrayLibrary.Array_Random` _spawnpoints)))
        (if (`self.IsPointUsed` _output_get)
          (goto _label)
          (else
            (bind _returnvalue (`|SpawnActorFromClass` (`KismetArrayLibrary.Array_Random` (`self.allRooms`)) (`KismetMathLibrary.Conv_VectorToTransform` (`self.currentPoint`)) "Undefined" "OverrideRootScale" null null))
            (`/Engine/EditorBlueprintResources/StandardMacros.IncrementInt` (`self.current`)
              (:`  `
                (`KismetArrayLibrary.Array_Add` (`self.spawnedPositions`) (`self.currentPoint`))
                (`KismetSystemLibrary.Delay` 1.0)
                (`self.Generate` _returnvalue)))))
        (else
          (`KismetSystemLibrary.PrintString` "Reached End")
          (set `self.current` (`self.limit`)))))))

(fn `IsPointUsed`
  (params (point :type "Vector Structure"))
  (returns (isUsed :type Boolean))
  (locals (used :type Boolean))
  (if (> (`KismetArrayLibrary.Array_Length` (`self.spawnedPositions`)) 0)
    (for _array_element (`self.spawnedPositions`)
      (if (== _array_element point :`ErrorTolerance` 0.1)
        (set `local.used` true)
        (break)
        (else
          (set `local.used` false))))
    (return (`local.used`))
    (else
      (return false))))

(fn `UserConstructionScript`)