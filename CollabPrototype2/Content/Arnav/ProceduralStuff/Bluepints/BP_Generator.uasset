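; Procedural level generator that builds a room layout by random walk from a spawn point, placing room actors from an indexed array.
; On BeginPlay it spawns a starting room, then a delayed loop calls Propogate to step right, left or down (+Y) within limits.
; Before moving down, a sphere overlap finds the current room and replaces unsuitable types with bottom-opening ones, using a counter for consecutive descents.
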(event `self.ReceiveBeginPlay`
  (`KismetSystemLibrary.DrawDebugSphere` (`self.spawnPoint`) 100.0 12 (struct :`R` 0.192751 :`G` 1.0 :`A` 1.0) 5.0 5.0) ; Start point
  (`self.SpawnRoomIndexed` 1) ; Spawn starting room (LR)
  (`self.Get New Direction` 1
    (:`execOut`
      (`/Game/Arnav/ActorMacroLibrary.For Loop with Delay` 0 10 1.0
        (:`Loop Body`
          (if (not (`self.stopPropogation`))
            (`self.Propogate`)
            (else
              (`KismetSystemLibrary.PrintString` "Over"))))
        (:`Completed`
          (`KismetSystemLibrary.PrintString` "-----      Done     -----" true true (struct :`R` 1.0 :`G` 0.01492 :`A` 1.0) 5.0))))))

(fn `MoveDown`
  (bind (_spawnpoint_x _spawnpoint_y _spawnpoint_z) (`KismetMathLibrary.BreakVector` (`self.spawnPoint`)))
  (set `self.spawnPoint` (`KismetMathLibrary.MakeVector` _spawnpoint_x (+ _spawnpoint_y (`self.propogationDistance`)) _spawnpoint_z)))

(fn `MoveLeft`
  (bind (_spawnpoint_x _spawnpoint_y _spawnpoint_z) (`KismetMathLibrary.BreakVector` (`self.spawnPoint`)))
  (set `self.spawnPoint` (`KismetMathLibrary.MakeVector` (- _spawnpoint_x (`self.propogationDistance`)) _spawnpoint_y _spawnpoint_z)))

(fn `MoveRight`
  (bind (_spawnpoint_x _spawnpoint_y _spawnpoint_z) (`KismetMathLibrary.BreakVector` (`self.spawnPoint`)))
  (set `self.spawnPoint` (`KismetMathLibrary.MakeVector` (+ _spawnpoint_x (`self.propogationDistance`)) _spawnpoint_y _spawnpoint_z)))

(fn `Propogate`
  (locals (previousRoom :type "Actor Object Reference") (downOpening :type Integer))
  (bind _spawnpoint_x (`KismetMathLibrary.BreakVector` (`self.spawnPoint`)))
  (bind _previousroom (`local.previousRoom`))
  (`KismetSystemLibrary.PrintString` (`KismetStringLibrary.Conv_IntToString` (`self.direction`)))
  (if (or (`self.Direction Equals` 1) (`self.Direction Equals` 2))
    (if (`self.In X Limit`)
      (set `self.moveDownCounter` 0) ; Reset down movement
      (`self.MoveRight`)
      (`self.SpawnRandomRoomInRange` 1)
      (`self.Get New Direction` 1
        (:`execOut`
          (if (`self.Direction Equals` 3)
            (set `self.direction` 1)
            (elif (`self.Direction Equals` 4)
              (set `self.direction` 5)))))
      (else
        (set `self.direction` 50)))
    (elif (or (`self.Direction Equals` 3) (`self.Direction Equals` 4))
      (if (> _spawnpoint_x 0.0)
        (set `self.moveDownCounter` 0)
        (`self.MoveLeft`)
        (`self.SpawnRandomRoomInRange` 1)
        (`self.Get New Direction` 3)
        (else
          (set `self.direction` 5)))
      (elif (`self.Direction Equals` 5)
        (`/Engine/EditorBlueprintResources/StandardMacros.IncrementInt` (`self.moveDownCounter`)
          (:`  `
            (if (`self.In Y Limit`)
              (bind _outactors (`KismetSystemLibrary.SphereOverlapActors` (`self.spawnPoint`) 250.0 (`|MakeArray` "ObjectTypeQuery1" "ObjectTypeQuery2" :!type "EObjectTypeQuery Enum")))
              (bind _output_get (set `local.previousRoom` (`|GetArrayItem` _outactors)))
              (cast `/Game/Arnav/ProceduralStuff/Rooms/BP_Room_Base_LRTB` _output_get ; Niether type 4 nor type 2
                (:`CastFailed`
                  (cast `/Game/Arnav/ProceduralStuff/Rooms/BP_Room_Base_LRB` _output_get
                    (:`CastFailed`
                      (if (> (`self.moveDownCounter`) 2)
                        (`self.K2_DestroyActor` _previousroom)
                        (`self.SpawnRoomIndexed` 4)
                        (else
                          (`self.K2_DestroyActor` _previousroom)
                          (bind _output_get_2 (set `local.downOpening` (`KismetMathLibrary.RandomIntegerInRange` 2 4)))
                          (if (== _output_get_2 3)
                            (set `local.downOpening` 2))
                          (`self.SpawnRoomIndexed` (`local.downOpening`))))
                      (`self.MoveDown`)
                      (`self.SpawnRandomRoomInRange` 3)
                      (`self.Get New Direction` 1)))))
              (else
                (set `self.stopPropogation` true)))))))))

(fn `SpawnRandomRoom`
  (returns (room :type "/Game/Arnav/ProceduralStuff/Rooms/BP_Room_Base Object Reference"))
  (bind _returnvalue (`|SpawnActorFromClass` (`self.Get Random Room`) (`KismetMathLibrary.Conv_VectorToTransform` (`self.spawnPoint`)) "Undefined" "OverrideRootScale" null null))
  (return _returnvalue))

(fn `SpawnRandomRoomInRange`
  (params (min :type Integer :default 1) (max :type Integer :default 4))
  (returns (room :type "/Game/Arnav/ProceduralStuff/Rooms/BP_Room_Base Object Reference") (index :type Integer))
  (bind _returnvalue (`KismetMathLibrary.RandomIntegerInRange` min max))
  (bind _returnvalue_2 (`|SpawnActorFromClass` (`|GetArrayItem` (`self.rooms`) _returnvalue) (`KismetMathLibrary.Conv_VectorToTransform` (`self.spawnPoint`)) "Undefined" "OverrideRootScale" null null))
  (return _returnvalue_2 _returnvalue))

(fn `SpawnRoomIndexed`
  (params (index :type Integer))
  (returns (room :type "/Game/Arnav/ProceduralStuff/Rooms/BP_Room_Base Object Reference"))
  (bind _returnvalue (`|SpawnActorFromClass` (`|GetArrayItem` (`self.rooms`) index) (`KismetMathLibrary.Conv_VectorToTransform` (`self.spawnPoint`)) "Undefined" "OverrideRootScale" null null))
  (return _returnvalue))

(fn `UserConstructionScript`)