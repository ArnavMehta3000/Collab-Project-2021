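; BP_Reader probes the grid cell next to a target actor for BP_RoomBase actors.
; Read computes a position one CellSize from TargetClass along MoveDirection, then runs a sphere overlap there filtered to rooms.
; Debug spheres mark the probed position.
; The loop over overlap results is empty, with an unconnected string append left for labelling hits, and the position update hangs off only the None output of DirectionToVector.
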(event `DrawSphere`
  (`KismetSystemLibrary.DrawDebugSphere` (`self.position`) 250.0 12 (struct :`R` 1.0 :`B` 0.217588 :`A` 1.0) 3.0 25.0))

(event `GetPosition`
  (bind _direction (`/Game/Arnav/Blueprints/Data/MyMacroLibrary.DirectionToVector` (`self.moveDirection`))
    (:`None`
      (bind _returnvalue (+ (`self.K2_GetActorLocation` (`self.targetClass`)) (* _direction (`self.cellSize`))))
      (`KismetSystemLibrary.DrawDebugSphere` _returnvalue 500.0 12 (struct :`G` 1.0 :`B` 0.226714 :`A` 1.0) 3.0 25.0)
      (set `self.position` _returnvalue)
      (`self.DrawSphere`))))

(event `Read`
  (`self.GetPosition`)
  (bind _outactors (`KismetSystemLibrary.SphereOverlapActors` (`self.position`) 250.0 (`|MakeArray` "ObjectTypeQuery1" "ObjectTypeQuery2" "ObjectTypeQuery3" :!type "EObjectTypeQuery Enum") "/Game/Arnav/Blueprints/Rooms/BP_RoomBase.BP_RoomBase_C"))
  (for (_array_element _array_index) _outactors
    _))

(fn `UserConstructionScript`)