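; Procedural level generator that builds a random chain of grid-aligned rooms on BeginPlay.
; From a random starting room, Propogate recursively picks connections from rule data tables, rejecting occupied cells and restarting generation when the attempt limit runs out.
; The final room uses a closed-room table and gets an end zone.
; Traverse then spawns doors midway between consecutive rooms, oriented by direction; DrawPath offers a debug line view.
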(event `self.ReceiveBeginPlay`
  (`self.Generate`))

(event `Cleanup`
  (bind _spawnedrooms (`self.spawnedRooms`))
  (bind _spawneddoors (`self.spawnedDoors`))
  (for _array_element _spawneddoors
    (`self.K2_DestroyActor` _array_element))
  (`KismetArrayLibrary.Array_Clear` _spawneddoors)
  (`KismetSystemLibrary.FlushDebugStrings`)
  (`KismetSystemLibrary.FlushPersistentDebugLines`)
  (bind _keys (`BlueprintMapLibrary.Map_Keys` _spawnedrooms))
  (for _array_element_2 _keys
    (`self.K2_DestroyActor` _array_element_2))
  (`BlueprintMapLibrary.Map_Clear` _spawnedrooms)
  (set `self.limit` 200)
  (set `self.positionPointer` (0.0 0.0 0.0))
  (set `self.flag` false)
  (set `self.spawnLimit` (`self.spawnCount`)))

(event `AddToList`
  (params (room :type "/Game/Arnav/Blueprints/Rooms/BP_RoomBase Object Reference") (fromDirection :type "/Game/Arnav/Blueprints/Data/E_MoveDirection Enum" :default "NewEnumerator0"))
  (`BlueprintMapLibrary.Map_Add` (`self.spawnedRooms`) room fromDirection))

(event `Generate`
  (`self.Cleanup`)
  (`self.SpawnFirst`)
  (`KismetSystemLibrary.PrintString` "Starting generation")
  (`self.Propogate` (`self.startingRoom`))
  (`KismetSystemLibrary.PrintString` "Begin Traversal")
  (bind _keys (`BlueprintMapLibrary.Map_Keys` (`self.spawnedRooms`)))
  (`self.Traverse` _keys))

(event `SpawnFirst`
  (bind _output_get (set `self.startingRoom` (`KismetArrayLibrary.Array_Random` (`self.staringRooms`))))
  (bind _returnvalue (`|SpawnActorFromClass` _output_get (`KismetMathLibrary.Conv_VectorToTransform` (`self.positionPointer`)) "Undefined" "OverrideRootScale" null null))
  (`self.AddToList` _returnvalue))

(fn `Draw Path`
  (locals (length :type Integer))
  (bind _returnvalue (`BlueprintMapLibrary.Map_Length` (`self.spawnedRooms`)))
  (`KismetSystemLibrary.PrintString` (`KismetStringLibrary.Concat_StrStr` "-----------------Completed Rooms: " (`KismetStringLibrary.Conv_IntToString` _returnvalue) " -----------------") true true (struct :`R` 0.049157 :`G` 1.0 :`A` 1.0))
  (bind _output_get (set `local.length` _returnvalue))
  (for _index (range _output_get)
    (bind _returnvalue_2 (+ _index 1))
    (if (== _returnvalue_2 (`local.length`))
      (break)
      (else
        (bind _keys (`BlueprintMapLibrary.Map_Keys` (`self.spawnedRooms`)))
        (bind (_returnvalue_x _returnvalue_y _returnvalue_z) (`KismetMathLibrary.BreakVector` (`self.K2_GetActorLocation` (`|GetArrayItem` _keys _returnvalue_2))))
        (bind (_returnvalue_x_2 _returnvalue_y_2 _returnvalue_z_2) (`KismetMathLibrary.BreakVector` (`self.K2_GetActorLocation` (`|GetArrayItem` _keys _index))))
        (`KismetSystemLibrary.DrawDebugLine` (`KismetMathLibrary.MakeVector` _returnvalue_x (+ _returnvalue_y 1000.0) _returnvalue_z) (`KismetMathLibrary.MakeVector` _returnvalue_x_2 (+ _returnvalue_y_2 1000.0) _returnvalue_z_2) (`self.debugPathColor`) (`self.pathDrawTime`) (`self.Thickness`))))))

(fn `GetPossibleRoomConnections`
  (params (room :type "/Game/Arnav/Blueprints/Rooms/BP_RoomBase Class Reference") (isSecondLast :type Boolean))
  (returns (possibleConnections :type "Array of /Game/Arnav/Blueprints/Data/S_NewRules Structure"))
  (locals (connections :type "Array of /Game/Arnav/Blueprints/Data/S_NewRules Structure"))
  (bind _returnvalue (select `bool` isSecondLast :`false` "/Game/Arnav/Blueprints/Data/NewRuleSet.NewRuleSet" :`true` "/Game/Arnav/Blueprints/Data/ClosedRoomRules.ClosedRoomRules" :!type "DataTable Object Reference"))
  (bind _outrownames (`DataTableFunctionLibrary.GetDataTableRowNames` _returnvalue))
  (for _array_element _outrownames
    (bind _returnvalue_2 (`|GetDataTableRow` _returnvalue _array_element)
      (:`then`
        (`/Game/Arnav/Blueprints/Data/MyMacroLibrary.IsRoomEqual` (`.From_5_1179DF6C439B149BD75641AD3EA38359` (break `/Game/Arnav/Blueprints/Data/S_NewRules` _returnvalue_2)) room
          (:`True`
            (`KismetArrayLibrary.Array_Add` (`local.connections`) _returnvalue_2))))))
  (return (`local.connections`)))

(fn `MoveDirectionFromTwoRooms`
  (params (fromRoom :type "Vector Structure") (toRoom :type "Vector Structure"))
  (returns (direction :type "/Game/Arnav/Blueprints/Data/E_MoveDirection Enum"))
  (locals (dirIndex :type Integer) (normalizedDir :type "Vector Structure" :default (0.0 0.0 0.0)))
  (bind _output_get (set `local.normalizedDir` (`KismetMathLibrary.Normal` (- toRoom fromRoom))))
  (if (== _output_get (-1.0 0.0 0.0))
    (set `local.dirIndex` 1)
    (elif (== _output_get (1.0 0.0 0.0))
      (set `local.dirIndex` 2)
      (elif (== _output_get (0.0 -1.0 0.0))
        (set `local.dirIndex` 3)
        (elif (== _output_get (0.0 1.0 0.0))
          (set `local.dirIndex` 4)))))
  (return (select `int` (`local.dirIndex`) :`0` "NewEnumerator0" :`1` "NewEnumerator1" :`2` "NewEnumerator2" :`3` "NewEnumerator3" :`4` "NewEnumerator4" :!type "/Game/Arnav/Blueprints/Data/E_MoveDirection Enum")))

(fn `Propogate`
  (params (fromClass :type "/Game/Arnav/Blueprints/Rooms/BP_RoomBase Class Reference"))
  (locals (newConnection :type "/Game/Arnav/Blueprints/Data/S_NewRules Structure"))
  (bind (_newconnection_from _newconnection_to _newconnection_movedirection) (break `/Game/Arnav/Blueprints/Data/S_NewRules` (`local.newConnection`)))
  (bind _returnvalue (`KismetMathLibrary.Conv_VectorToTransform` (`self.positionPointer`)))
  (bind _is_1 (`self.CanPropogate` :!label _label)
    (:`true`
      (`/Engine/EditorBlueprintResources/StandardMacros.DecrementInt` (`self.limit`)
        (:`  `
          (bind _output_get (set `local.newConnection` (`self.GetRandomConnection` (`self.GetPossibleRoomConnections` fromClass _is_1))))
          (`self.CheckNewPositionIsValid` (`.MoveDirection_11_250F50464EFBC3AC1FA2DCA9FB0775BD` (break `/Game/Arnav/Blueprints/Data/S_NewRules` _output_get)) true
            (:`True`
              (bind _returnvalue_2 (`|SpawnActorFromClass` _newconnection_to _returnvalue "Undefined" "OverrideRootScale" null null))
              (if _is_1
                (`|SpawnActorFromClass` "/Game/Rowan/tempendzone.tempendzone_C" (`KismetMathLibrary.MakeTransform` (.location _returnvalue) (.rotation _returnvalue)) "Undefined" "OverrideRootScale" null null))
              (`self.AddToList` _returnvalue_2 _newconnection_movedirection)
              (bind _asroom_manager (cast `/Game/Rowan/Room_Manager` (`|GetArrayItem` (`self.GetAllChildActors` _returnvalue_2 false))))
              (set `/Game/Rowan/Room_Manager.Room Number` (`BlueprintMapLibrary.Map_Length` (`self.spawnedRooms`)) _asroom_manager)
              (`/Engine/EditorBlueprintResources/StandardMacros.DecrementInt` (`self.spawnLimit`)
                (:`  `
                  (`self.Propogate` _newconnection_to))))
            (:`False`
              (goto _label))))))
    (:`LimitReached`
      (`self.Cleanup`)
      (`self.Generate`))))

(fn `RoomClassToEnum`
  (params (roomClass :type "/Game/Arnav/Blueprints/Rooms/BP_RoomBase Class Reference"))
  (returns (roomType :type "/Game/Arnav/Blueprints/Data/E_RoomType Enum"))
  ;[1 1 1] Check Singles
  (`/Game/Arnav/Blueprints/Data/MyMacroLibrary.IsRoomEqual` roomClass "/Game/Arnav/Blueprints/Rooms/Single/BP_RoomL.BP_RoomL_C"
    (:`True`
      (return "NewEnumerator0"))
    (:`False`
      (`/Game/Arnav/Blueprints/Data/MyMacroLibrary.IsRoomEqual` roomClass "/Game/Arnav/Blueprints/Rooms/Single/BP_RoomR.BP_RoomR_C"
        (:`True`
          (return "NewEnumerator1"))
        (:`False`
          (`/Game/Arnav/Blueprints/Data/MyMacroLibrary.IsRoomEqual` roomClass "/Game/Arnav/Blueprints/Rooms/Single/BP_RoomT.BP_RoomT_C"
            (:`True`
              (return "NewEnumerator2"))
            (:`False`
              (`/Game/Arnav/Blueprints/Data/MyMacroLibrary.IsRoomEqual` roomClass "/Game/Arnav/Blueprints/Rooms/Single/BP_RoomB.BP_RoomB_C"
                (:`True`
                  (return "NewEnumerator3"))
                (:`False`
                  ;[1 1 1] Check Doubles
                  (`/Game/Arnav/Blueprints/Data/MyMacroLibrary.IsRoomEqual` roomClass "/Game/Arnav/Blueprints/Rooms/Double/BP_RoomLB.BP_RoomLB_C"
                    (:`True`
                      (return "NewEnumerator6"))
                    (:`False`
                      (`/Game/Arnav/Blueprints/Data/MyMacroLibrary.IsRoomEqual` roomClass "/Game/Arnav/Blueprints/Rooms/Double/BP_RoomLR.BP_RoomLR_C"
                        (:`True`
                          (return "NewEnumerator5"))
                        (:`False`
                          (`/Game/Arnav/Blueprints/Data/MyMacroLibrary.IsRoomEqual` roomClass "/Game/Arnav/Blueprints/Rooms/Double/BP_RoomLT.BP_RoomLT_C"
                            (:`True`
                              (return "NewEnumerator7"))
                            (:`False`
                              (`/Game/Arnav/Blueprints/Data/MyMacroLibrary.IsRoomEqual` roomClass "/Game/Arnav/Blueprints/Rooms/Double/BP_RoomRB.BP_RoomRB_C"
                                (:`True`
                                  (return "NewEnumerator8"))
                                (:`False`
                                  (`/Game/Arnav/Blueprints/Data/MyMacroLibrary.IsRoomEqual` roomClass "/Game/Arnav/Blueprints/Rooms/Double/BP_RoomRT.BP_RoomRT_C"
                                    (:`True`
                                      (return "NewEnumerator9"))
                                    (:`False`
                                      (`/Game/Arnav/Blueprints/Data/MyMacroLibrary.IsRoomEqual` roomClass "/Game/Arnav/Blueprints/Rooms/Double/BP_RoomTB.BP_RoomTB_C"
                                        (:`True`
                                          (return "NewEnumerator10"))))))))))))))))))))))

(fn `Traverse`
  (params (rooms :type "Array of /Game/Arnav/Blueprints/Rooms/BP_RoomBase Object Reference"))
  (locals (index :type Integer))
  (bind _returnvalue (`KismetArrayLibrary.Array_Length` rooms))
  (bind _spawneddoors (`self.spawnedDoors`))
  (for _index (range _returnvalue)
    (bind _returnvalue_2 (+ _index 1))
    (if (== _returnvalue_2 _returnvalue)
      (break)
      (else
        (bind _returnvalue_3 (`self.K2_GetActorLocation` (`|GetArrayItem` rooms _index)))
        (bind _returnvalue_4 (`self.K2_GetActorLocation` (`|GetArrayItem` rooms _returnvalue_2)))
        (bind _direction (`self.MoveDirectionFromTwoRooms` _returnvalue_3 _returnvalue_4))
        (switch `/Game/Arnav/Blueprints/Data/E_MoveDirection` _direction
          (:`NewEnumerator1`
            (bind _midpoint (`self.GetMidPoint` _returnvalue_3 _returnvalue_4))
            (bind _returnvalue_5 (`|SpawnActorFromClass` "/Game/Arnav/Blueprints/Doors/BP_DoorBase.BP_DoorBase_C" (`KismetMathLibrary.MakeTransform` _midpoint) "Undefined" "OverrideRootScale" null null :!label _label))
            (`KismetArrayLibrary.Array_Add` _spawneddoors _returnvalue_5))
          (:`NewEnumerator2`
            (goto _label))
          (:`NewEnumerator3`
            (bind _returnvalue_6 (`|SpawnActorFromClass` "/Game/Arnav/Blueprints/Doors/BP_DoorBase.BP_DoorBase_C" (`KismetMathLibrary.MakeTransform` _midpoint (struct :`Yaw` 90.0)) "Undefined" "OverrideRootScale" null null :!label _label_2))
            (`KismetArrayLibrary.Array_Add` _spawneddoors _returnvalue_6))
          (:`NewEnumerator4`
            (goto _label_2)))))))

(fn `UserConstructionScript`)