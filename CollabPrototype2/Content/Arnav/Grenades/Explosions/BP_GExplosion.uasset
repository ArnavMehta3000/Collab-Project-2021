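; BP_GExplosion is a grenade explosion actor that applies area damage and a physics push when it spawns.
; On BeginPlay it widens its sphere to a large radius and sends an IHitMessage with fixed damage to every overlapping actor, without filtering.
; The first FirstPersonCharacterROwan found in the world is passed as instigator.
; It then fires a RadialForce impulse and sets a short lifespan to remove itself.
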(event `self.ReceiveBeginPlay`
  (bind _returnvalue (`GameplayStatics.GetActorOfClass` "/Game/Rowan/FirstPersonCharacterROwan.FirstPersonCharacterROwan_C"))
  (set `self.Player` _returnvalue)
  (`SphereComponent.SetSphereRadius` (`self.Sphere`) 2000.0 true)
  (for _array_element (`PrimitiveComponent.GetOverlappingActors` (`self.Sphere`) null)
    (message `/Game/Rowan/I_Hit.I_Hit` _array_element (`self.Player`) 20.0))
  (`RadialForceComponent.FireImpulse` (`self.RadialForce`))
  (`self.SetLifeSpan` 3.0))

(fn `UserConstructionScript`)