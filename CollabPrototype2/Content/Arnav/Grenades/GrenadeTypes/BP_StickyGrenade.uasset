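; BP_StickyGrenade is a grenade that stays where it first hits, then explodes.
; The first hit on its static mesh turns off physics simulation, guarded by a DoOnce; it is not attached to the hit object.
; BeginPlay defers to the parent, which is noted as calling Detonate.
; Detonate spawns BP_GExplosion at the grenade's transform and destroys the grenade.
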(event `self.ReceiveBeginPlay`
  (`parent.ReceiveBeginPlay`) ; Calls detonate
)

(event `self.StaticMesh.OnComponentHit`
  (params (HitComponent :type "PrimitiveComponent Object Reference") (OtherActor :type "Actor Object Reference") (OtherComp :type "PrimitiveComponent Object Reference") (NormalImpulse :type "Vector Structure") (Hit :type "HitResult Structure (by ref)"))
  (`/Engine/EditorBlueprintResources/StandardMacros.DoOnce` false
    (:`Completed`
      (`PrimitiveComponent.SetSimulatePhysics` (`self.StaticMesh`) false) ; Stop simulating when hit something
    )))

(fn `Detonate`
  (`|SpawnActorFromClass` "/Game/Arnav/Grenades/Explosions/BP_GExplosion.BP_GExplosion_C" (`self.GetTransform`) "Undefined" "OverrideRootScale" null null)
  (`self.K2_DestroyActor`))

(fn `UserConstructionScript`
  (`parent.UserConstructionScript`))