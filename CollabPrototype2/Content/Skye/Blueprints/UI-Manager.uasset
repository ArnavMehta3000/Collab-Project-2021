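; UI manager actor that creates the in-game HUD and fills it with the player's starting state.
; Its Init event spawns the InGameUI widget, adds it to the viewport and registers itself as UIManager on the player character reference obtained through an interface message.
; It then passes the supplied values to child widgets for three abilities, health and portrait, ammo and gun image, and combo text.
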(event `Init`
  (params (`Ability 1` :type "/Game/Skye/Structs/S_InitAbilityUI Structure") (`Ability 2` :type "/Game/Skye/Structs/S_InitAbilityUI Structure") (`Ability 3` :type "/Game/Skye/Structs/S_InitAbilityUI Structure") (`Player HP` :type "/Game/Skye/Structs/S_HP Structure") (`Player PFP` :type "Texture2D Object Reference") (`Ammo Count` :type "/Game/Skye/Structs/S_Ammo Structure") (`Gun PFP` :type "Texture2D Object Reference") (ComboText :type Text))
  (bind _ingameui (`self.InGameUI`))
  (bind _playerhealthui (`/Game/Skye/UIBlueprints/InGameUI.PlayerHealthUI` _ingameui))
  (bind _ammocounterui (`/Game/Skye/UIBlueprints/InGameUI.AmmoCounterUI` _ingameui))
  (`|ExecutionSequence`
    (:`then_0`
      (bind _returnvalue (`|CreateWidget` "/Game/Skye/UIBlueprints/InGameUI.InGameUI_C"))
      (bind _output_get (set `self.InGameUI` _returnvalue))
      (`UserWidget.AddToViewport` _output_get 0)
      (bind _newparam (message `/Game/FirstPersonBP/Rowan/I_Cast.I_Get Player Character` (`GameplayStatics.GetPlayerCharacter` 0)))
      (set `/Game/FirstPersonBP/Rowan/FirstPersonCharacterROwan.UI-Manager` self _newparam))
    (:`then_1`
      (`/Game/Skye/UIBlueprints/SubWidgets/AbilityUI.Init` (`/Game/Skye/UIBlueprints/InGameUI.Ability1UI` _ingameui) `Ability 1`)
      (`/Game/Skye/UIBlueprints/SubWidgets/AbilityUI.Init` (`/Game/Skye/UIBlueprints/InGameUI.Ability2UI` _ingameui) `Ability 2`)
      (`/Game/Skye/UIBlueprints/SubWidgets/AbilityUI.Init` (`/Game/Skye/UIBlueprints/InGameUI.Ability3UI` _ingameui) `Ability 3`))
    (:`then_2`
      (`/Game/Skye/UIBlueprints/SubWidgets/HealthUI.UpdateHPBar` _playerhealthui `Player HP`)
      (`/Game/Skye/UIBlueprints/SubWidgets/HealthUI.SetPFP` _playerhealthui `Player PFP`))
    (:`then_3`
      (`/Game/Skye/UIBlueprints/SubWidgets/AmmoCounterUI.Set Ammo` _ammocounterui `Ammo Count`)
      (`/Game/Skye/UIBlueprints/SubWidgets/AmmoCounterUI.Set Gun PFP` _ammocounterui `Gun PFP`))
    (:`then_4`
      (`/Game/Skye/UIBlueprints/SubWidgets/ComboUI.SetComboText` (`/Game/Skye/UIBlueprints/InGameUI.ComboUI` _ingameui) ComboText))))

(fn `UserConstructionScript`)