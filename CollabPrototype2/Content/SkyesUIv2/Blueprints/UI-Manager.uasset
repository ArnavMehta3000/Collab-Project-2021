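; UI manager that creates and updates the game's loading screen, lobby UI, in-game HUD and pause menu.
; Events push HP, score, abilities, ammo, enemy count, map and notifications into child widgets, while the pause toggle also sets game pause and input mode.
; A gated Tick drains the trailing damage bar after hits.
; A spawned Timeline_NoDilation_Actor, resized to each reload's duration, drives the reload bar.
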(event `StartLoadingScreen`
  (bind _returnvalue (`|CreateWidget` "/Game/SkyesUIv2/Blueprints/UI/LoadingScreenUI.LoadingScreenUI_C"))
  (bind _output_get (set `self.LoadingScreen` _returnvalue))
  (`UserWidget.PlayAnimation` _output_get (`/Game/SkyesUIv2/Blueprints/UI/LoadingScreenUI.OPACITYBITCHV2` _output_get) 0.0 1 "Forward" 1.0 false)
  (`UserWidget.AddToViewport` _output_get 999999)
  (`WidgetBlueprintLibrary.SetInputMode_UIOnlyEx` (`GameplayStatics.GetPlayerController` 0) null))

(event `LoadOutLoadingScreen`
  (bind _loadingscreen (`self.LoadingScreen`))
  (bind _opacitybitchv2 (`/Game/SkyesUIv2/Blueprints/UI/LoadingScreenUI.OPACITYBITCHV2` _loadingscreen))
  (bind _returnvalue (`|CreateWidget` "/Game/SkyesUIv2/Blueprints/UI/LoadingScreenUI.LoadingScreenUI_C"))
  (bind _output_get (set `self.LoadingScreen` _returnvalue))
  (`UserWidget.AddToViewport` _output_get 999999)
  (`KismetSystemLibrary.Delay` 2.0)
  (`UserWidget.PlayAnimation` _loadingscreen _opacitybitchv2 0.0 1 "Reverse" 1.0 false)
  (`KismetSystemLibrary.Delay` (`WidgetAnimation.GetEndTime` _opacitybitchv2))
  (`Widget.RemoveFromParent` (`self.LoadingScreen`))
  (`WidgetBlueprintLibrary.SetInputMode_GameOnly` (`GameplayStatics.GetPlayerController` 0)))

(event `ExampleUpdate`
  ;[1 1 1] Timeline base shits
)

(event `ExampleFinished`
  ;[1 1 1] Timeline base shits
)

(event `InLobbyUI Init`
  ;[1 1 1] InLobbyINIT
  (bind _game_instance (message `/Game/Rowan/I_Cast.I_Get Game Instance` (`GameplayStatics.GetGameInstance`)))
  (bind _returnvalue (`|CreateWidget` "/Game/SkyesUIv2/Blueprints/UI/InLobbyUI.InLobbyUI_C"))
  (bind _output_get (set `self.InLobbyUI` _returnvalue))
  (`UserWidget.AddToViewport` _output_get 0)
  (`self.SetScoreInLobby` (`/Game/Rowan/Cyber_Instance.Score` _game_instance))
  (`self.GenPauseMenuUI` "NewEnumerator3"))

(event `SetScoreInLobby`
  (params (Score :type Integer))
  ;[1 1 1] Set Score Text In Lobby
  (`TextBlock.SetText` (`/Game/SkyesUIv2/Blueprints/UI/Widgets/W_PlayerScore.ScoreText` (`/Game/SkyesUIv2/Blueprints/UI/InLobbyUI.W_PlayerScore` (`self.InLobbyUI`))) (`KismetTextLibrary.Conv_IntToText` Score)))

(event `self.ReceiveTick`
  (params (DeltaSeconds :type "Float (single-precision)"))
  ;[1 1 1] Tick
  (`self.PlayerHPBarTick`))

(event `SpawnTimelines`
  ;[1 1 1] Timeline For Reload
  (bind _returnvalue (`|SpawnActorFromClass` "/Game/SkyesUIv2/Blueprints/Rowan-TimelineShits/Timeline_NoDilation_Actor.Timeline_NoDilation_Actor_C" (`KismetMathLibrary.MakeTransform` (0.0 0.0 0.0)) "Undefined" "OverrideRootScale" null 0.0 null))
  (bind _output_get (set `self.ReloadingTimeline` _returnvalue))
  (add `/Game/SkyesUIv2/Blueprints/Rowan-TimelineShits/Timeline_NoDilation_Actor.OnUpdate` _output_get (`|CreateDelegate` :!event `ReloadTimerUpdate`))
  (add `/Game/SkyesUIv2/Blueprints/Rowan-TimelineShits/Timeline_NoDilation_Actor.OnFinished` _output_get (`|CreateDelegate` :!event `ReloadTimerFinished`)))

(event `GenPauseMenuUI`
  (params (WhereBeingCalledFrom :type "/Game/SkyesUIv2/Blueprints/Enums/E_WherePauseCalledFrom Enum" :default "NewEnumerator0"))
  ;[1 1 1] Gen Pause Menu
  (bind _returnvalue (`|CreateWidget` "/Game/SkyesUIv2/Blueprints/UI/PauseMenuUI.PauseMenuUI_C" null WhereBeingCalledFrom))
  (`UserWidget.AddToViewport` _returnvalue 0)
  (bind _output_get (set `self.PauseMenuUI` _returnvalue))
  (`Widget.SetVisibility` _output_get "Hidden"))

(event `InGameUI Init`
  (params (CurrentHP :type "Float (double-precision)") (MaxHP :type "Float (double-precision)"))
  (bind _w_playerhp (`/Game/SkyesUIv2/Blueprints/UI/InGameUI.W_PlayerHP` (`self.InGameUI`)))
  ;[1 1 1] InGameUI Init
  (bind _returnvalue (`|CreateWidget` "/Game/SkyesUIv2/Blueprints/UI/InGameUI.InGameUI_C"))
  (bind _output_get (set `self.InGameUI` _returnvalue))
  (`UserWidget.AddToViewport` _output_get 0)
  (`|ExecutionSequence`
    (:`then_0`
      (set `self.Effect HPBar` (`/Game/SkyesUIv2/Blueprints/UI/Widgets/W_PlayerHP.EffectHPBar` _w_playerhp))
      (set `self.Player HPBar` (`/Game/SkyesUIv2/Blueprints/UI/Widgets/W_PlayerHP.PlayerHPBar` _w_playerhp))
      (set `self.HPText` (`/Game/SkyesUIv2/Blueprints/UI/Widgets/W_PlayerHP.HPText` _w_playerhp)))
    (:`then_1`
      (`self.SpawnTimelines`))
    (:`then_2`
      (`self.SetupPlayerHP` CurrentHP MaxHP)
      (`self.SetScoreInGame` 0)
      (`self.SetEnemiesRemaining` 0)
      (`self.GenPauseMenuUI` "NewEnumerator0"))))

(event `SetupPlayerHP`
  (params (CurrentHP :type "Float (double-precision)") (MaxHP :type "Float (double-precision)"))
  ;[1 1 1] Setup Player HP
  (bind _progressbarvalue (`self.Map Range Clamped To Progress Bar` CurrentHP 0.0 MaxHP))
  (`ProgressBar.SetPercent` (`self.Effect HPBar`) _progressbarvalue)
  (`ProgressBar.SetPercent` (`self.Player HPBar`) _progressbarvalue))

(event `PlayerHPBarTick`
  (bind _currenthp_beforedamage (`self.CurrentHP BeforeDamage`))
  ;[1 1 1] Player Takes Damage
  (`/Engine/EditorBlueprintResources/StandardMacros.Gate` true :!label _label
    (:`Exit`
      (if (> _currenthp_beforedamage (stale `PlayerTakesDamage` CurrentHP))
        (bind _output_get (set `self.CurrentHP BeforeDamage` (- _currenthp_beforedamage (`self.HPBarEffectTime`))))
        (bind _progressbarvalue (`self.Map Range Clamped To Progress Bar` _output_get 0.0 (stale `PlayerTakesDamage` MaxHP)))
        (`ProgressBar.SetPercent` (`self.Effect HPBar`) _progressbarvalue)
        (else
          (bind _output_get_2 (set `self.CurrentHP BeforeDamage` (stale `PlayerTakesDamage` CurrentHP)))
          (`|ExecutionSequence`
            (:`then_0`
              (bind _progressbarvalue_2 (`self.Map Range Clamped To Progress Bar` _output_get_2 0.0 (stale `PlayerTakesDamage` MaxHP)))
              (`ProgressBar.SetPercent` (`self.Effect HPBar`) _progressbarvalue_2))
            (:`then_1`
              (goto _label :!via `Close`))))))))

(event `AbilityInit`
  (params (Abilities :type "Array of /Game/SkyesUIv2/Blueprints/Structs/S_AbilityDetails Structure"))
  ;[1 1 1] Inits the Abilities
  (for _array_element Abilities
    (bind _returnvalue (`|CreateWidget` "/Game/SkyesUIv2/Blueprints/UI/Widgets/W_Abilities.W_Abilities_C"))
    (`PanelWidget.AddChild` (`/Game/SkyesUIv2/Blueprints/UI/InGameUI.AbilitesBox` (`self.InGameUI`)) _returnvalue)
    (`KismetArrayLibrary.Array_AddUnique` (`self.AbilityUIWidgets`) _returnvalue)
    (`UserWidget.SetPadding` _returnvalue (make `Margin` 4.0 0.0 4.0))
    (bind (_doesabilityhaveuses_ _maxnumberofuses _abilityimage _abilitykeybind) (break `/Game/SkyesUIv2/Blueprints/Structs/S_AbilityDetails` _array_element))
    (`TextBlock.SetText` (`/Game/SkyesUIv2/Blueprints/UI/Widgets/W_Abilities.KeybindText` _returnvalue) _abilitykeybind)
    (`Image.SetBrushFromTexture` (`/Game/SkyesUIv2/Blueprints/UI/Widgets/W_Abilities.AbilityIcon` _returnvalue) _abilityimage false)
    (if _doesabilityhaveuses_
      (bind _abilityuseslefttext (`/Game/SkyesUIv2/Blueprints/UI/Widgets/W_Abilities.AbilityUsesLeftText` _returnvalue))
      (`Widget.SetVisibility` _abilityuseslefttext "HitTestInvisible")
      (`TextBlock.SetText` _abilityuseslefttext (`KismetTextLibrary.Conv_IntToText` _maxnumberofuses)))))

(event `PlayerTakesDamage`
  (params (CurrentHP :type "Float (double-precision)") (MaxHP :type "Float (double-precision)") (DamageAmount :type "Float (double-precision)"))
  ;[1 1 1] Player Takes Damage
  (bind _progressbarvalue (`self.Map Range Clamped To Progress Bar` CurrentHP 0.0 MaxHP))
  (`ProgressBar.SetPercent` (`self.Player HPBar`) _progressbarvalue)
  (set `self.CurrentHP BeforeDamage` (+ CurrentHP DamageAmount))
  (`TextBlock.SetText` (`self.HPText`) (`KismetTextLibrary.Conv_StringToText` (`KismetStringLibrary.Concat_StrStr` (`KismetStringLibrary.Conv_IntToString` (`KismetMathLibrary.FTrunc` CurrentHP)) " / " (`KismetStringLibrary.Conv_IntToString` (`KismetMathLibrary.FTrunc` MaxHP)))))
  (goto _label :!via `Open`))

(event `AbilityToRechage`
  (params (AbilityToUse :type Integer) (HowLongDoesItTake :type "Float (double-precision)"))
  ;[1 1 1] Ability UI Events
  (bind _abilitywidget (`self.GetAbilityUIWidget` AbilityToUse))
  (`/Game/SkyesUIv2/Blueprints/UI/Widgets/W_Abilities.AbilityRecharge` _abilitywidget HowLongDoesItTake))

(event `SetUltimateBar`
  (params (`Ultimate Gauge` :type "Float (double-precision)"))
  ;[1 1 1] Ultimate
  (bind _abilitywidget (`self.GetAbilityUIWidget` 4))
  (bind _progressbarvalue (`self.Map Range Clamped To Progress Bar` `Ultimate Gauge` 0.0 100.0))
  (bind _rechargebar (`/Game/SkyesUIv2/Blueprints/UI/Widgets/W_Abilities.RechargeBar` _abilitywidget))
  (`ProgressBar.SetPercent` _rechargebar _progressbarvalue)
  (`Widget.SetVisibility` _rechargebar "SelfHitTestInvisible"))

(event `PlayerHealed`
  (params (CurrentHP :type "Float (double-precision)") (MaxHP :type "Float (double-precision)"))
  ;[1 1 1] Player Healed
  (bind _progressbarvalue (`self.Map Range Clamped To Progress Bar` CurrentHP 0.0 MaxHP))
  (`ProgressBar.SetPercent` (`self.Player HPBar`) _progressbarvalue)
  (`ProgressBar.SetPercent` (`self.Effect HPBar`) _progressbarvalue)
  (`TextBlock.SetText` (`self.HPText`) (`KismetTextLibrary.Conv_StringToText` (`KismetStringLibrary.Concat_StrStr` (`KismetStringLibrary.Conv_IntToString` (`KismetMathLibrary.FTrunc` CurrentHP)) " / " (`KismetStringLibrary.Conv_IntToString` (`KismetMathLibrary.FTrunc` MaxHP))))))

(event `SetAbilityUsesText`
  (params (AbilityUsed :type Integer) (AmountLeft :type Integer))
  ;[1 1 1] Ability UI Events
  (bind _abilitywidget (`self.GetAbilityUIWidget` AbilityUsed))
  (`/Engine/EditorBlueprintResources/StandardMacros.IsValid` _abilitywidget
    (:`Is Valid`
      (`/Game/SkyesUIv2/Blueprints/UI/Widgets/W_Abilities.SetAbilityUsesText` _abilitywidget (`KismetTextLibrary.Conv_IntToText` AmountLeft)))))

(event `SetKeybindText`
  (params (AbilityKeybindIsFor :type Integer) (Key :type Text))
  ;[1 1 1] Ability UI Events
  (bind _abilitywidget (`self.GetAbilityUIWidget` AbilityKeybindIsFor))
  (`/Game/SkyesUIv2/Blueprints/UI/Widgets/W_Abilities.SetKeybindText` _abilitywidget Key))

(event `SetScoreInGame`
  (params (Score :type Integer))
  ;[1 1 1] Set Score In Game
  (`TextBlock.SetText` (`/Game/SkyesUIv2/Blueprints/UI/Widgets/W_PlayerScore.ScoreText` (`/Game/SkyesUIv2/Blueprints/UI/InGameUI.W_PlayerScore` (`self.InGameUI`))) (`KismetTextLibrary.Conv_IntToText` Score)))

(event `RemoveNotification`
  (params (Notification :type "/Game/SkyesUIv2/Blueprints/UI/Widgets/W_NotificationsAlert Object Reference"))
  ;[1 1 1] Notifications
  (`PanelWidget.RemoveChild` (`/Game/SkyesUIv2/Blueprints/UI/InGameUI.NotificationsBox` (`self.InGameUI`)) Notification))

(event `SetEnemiesRemaining`
  (params (`Total Number` :type Integer))
  ;[1 1 1] Set Enemies Remaining
  (`TextBlock.SetText` (`/Game/SkyesUIv2/Blueprints/UI/Widgets/W_EnemiesRemainingCounter.EnemiesRemainingText` (`/Game/SkyesUIv2/Blueprints/UI/InGameUI.W_EnemiesRemainingCounter` (`self.InGameUI`))) (`KismetTextLibrary.Conv_IntToText` `Total Number`)))

(event `SetWeaponImage`
  (params (Image :type "Texture2D Object Reference"))
  ;[1 1 1] Set Weapon Stuff
  (`Image.SetBrushFromTexture` (`/Game/SkyesUIv2/Blueprints/UI/Widgets/W_WeaponAndAmmo.WeaponImageOutline` (`/Game/SkyesUIv2/Blueprints/UI/InGameUI.W_WeaponAndAmmo` (`self.InGameUI`))) Image false))

(event `SetRemaingAmmoText`
  (params (`Remaining Ammo` :type Integer))
  ;[1 1 1] Set Weapon Stuff
  (`TextBlock.SetText` (`/Game/SkyesUIv2/Blueprints/UI/Widgets/W_WeaponAndAmmo.RemainingAmmo` (`/Game/SkyesUIv2/Blueprints/UI/InGameUI.W_WeaponAndAmmo` (`self.InGameUI`))) (`KismetTextLibrary.Conv_IntToText` `Remaining Ammo`)))

(event `SetCurrentAmmoText`
  (params (`Current Ammo` :type Integer))
  ;[1 1 1] Set Weapon Stuff
  (`TextBlock.SetText` (`/Game/SkyesUIv2/Blueprints/UI/Widgets/W_WeaponAndAmmo.CurrentAmmo` (`/Game/SkyesUIv2/Blueprints/UI/InGameUI.W_WeaponAndAmmo` (`self.InGameUI`))) (`KismetTextLibrary.Conv_IntToText` `Current Ammo`)))

(event `ToggleMap`
  (params (`ShowMap?` :type Boolean))
  (bind _w_map (`/Game/SkyesUIv2/Blueprints/UI/InGameUI.W_Map` (`self.InGameUI`)))
  (bind _displaymap (`/Game/SkyesUIv2/Blueprints/UI/Widgets/W_Map.DisplayMap` _w_map))
  ;[1 1 1] Toggle Map
  (if `ShowMap?`
    (`UserWidget.PlayAnimation` _w_map _displaymap 0.0 1 "Reverse" 1.0 false)
    (else
      (`UserWidget.PlayAnimation` _w_map _displaymap 0.0 1 "Forward" 1.0 false))))

(event `Reloading`
  (params (HowLongIsReload :type "Float (double-precision)"))
  (bind _any_internal_timeline (`/Game/SkyesUIv2/Blueprints/Rowan-TimelineShits/Timeline_NoDilation_Actor.Any Internal TimeLine` (`self.ReloadingTimeline`)))
  ;[1 1 1] Reloading
  (`TimelineComponent.SetTimelineLength` _any_internal_timeline HowLongIsReload) ; New Length is how long you want it to run for
  (`TimelineComponent.PlayFromStart` _any_internal_timeline)
  (`Widget.SetVisibility` (`/Game/SkyesUIv2/Blueprints/UI/InGameUI.W_Reload` (`self.InGameUI`)) "HitTestInvisible"))

(event `ReloadTimerUpdate`
  ;[1 1 1] Reloading
  (bind _progressbarvalue (`self.Map Range Clamped To Progress Bar` (`TimelineComponent.GetPlaybackPosition` (`/Game/SkyesUIv2/Blueprints/Rowan-TimelineShits/Timeline_NoDilation_Actor.Any Internal TimeLine` (`self.ReloadingTimeline`))) (stale `Reloading` HowLongIsReload)))
  (`ProgressBar.SetPercent` (`/Game/SkyesUIv2/Blueprints/UI/Widgets/W_Reload.ReloadBar` (`/Game/SkyesUIv2/Blueprints/UI/InGameUI.W_Reload` (`self.InGameUI`))) _progressbarvalue))

(event `TogglePauseMenu`
  (params (ShowPauseMenu :type Boolean) (WherePauseCalledFrom :type "/Game/SkyesUIv2/Blueprints/Enums/E_WherePauseCalledFrom Enum" :default "NewEnumerator0"))
  (bind _returnvalue (`GameplayStatics.GetPlayerController` 0))
  (bind _returnvalue_2 (`GameplayStatics.GetPlayerController` 0))
  (bind _returnvalue_3 (`GameplayStatics.GetPlayerController` 0))
  (bind _returnvalue_4 (`GameplayStatics.GetPlayerController` 0))
  (bind _pausemenuui (`self.PauseMenuUI`))
  (bind _pausemenuui_2 (`self.PauseMenuUI`))
  ;[1 1 1] Pause
  (switch `/Game/SkyesUIv2/Blueprints/Enums/E_WherePauseCalledFrom` WherePauseCalledFrom
    (:`NewEnumerator0`
      (if ShowPauseMenu
        (`GameplayStatics.SetGamePaused` true)
        (`Widget.SetVisibility` _pausemenuui "Visible")
        (set `PlayerController.bShowMouseCursor` true _returnvalue_3)
        (`WidgetBlueprintLibrary.SetInputMode_UIOnlyEx` _returnvalue_3 _pausemenuui)
        (`TextBlock.SetText` (`/Game/SkyesUIv2/Blueprints/UI/PauseMenuUI.ExtraButtonText` _pausemenuui) "Go to Lobby")
        (else
          (`GameplayStatics.SetGamePaused` false)
          (`Widget.SetVisibility` (`self.PauseMenuUI`) "Hidden")
          (set `PlayerController.bShowMouseCursor` false _returnvalue_4)
          (`WidgetBlueprintLibrary.SetInputMode_GameOnly` _returnvalue_4))))
    (:`NewEnumerator3`
      (if ShowPauseMenu
        (`GameplayStatics.SetGamePaused` true)
        (`Widget.SetVisibility` _pausemenuui_2 "Visible")
        (set `PlayerController.bShowMouseCursor` true _returnvalue_2)
        (`WidgetBlueprintLibrary.SetInputMode_UIOnlyEx` _returnvalue_2 _pausemenuui_2)
        (`TextBlock.SetText` (`/Game/SkyesUIv2/Blueprints/UI/PauseMenuUI.ExtraButtonText` _pausemenuui_2) "Go to Main Menu")
        (else
          (`GameplayStatics.SetGamePaused` false)
          (`Widget.SetVisibility` (`self.PauseMenuUI`) "Hidden")
          (set `PlayerController.bShowMouseCursor` false _returnvalue)
          (`WidgetBlueprintLibrary.SetInputMode_GameOnly` _returnvalue))))))

(event `ReloadTimerFinished`
  ;[1 1 1] Reloading
  (`Widget.SetVisibility` (`/Game/SkyesUIv2/Blueprints/UI/InGameUI.W_Reload` (`self.InGameUI`)) "Hidden"))

(fn `GetAbilityImage`
  (params (Ability :type "/Game/Rowan/E_Abilities Enum" :default "NewEnumerator8"))
  (returns (`Ability Image` :type "Texture2D Object Reference"))
  (return (`BlueprintMapLibrary.Map_Find` (`self.Ability Image Map`) Ability)))

(fn `GetAbilityUIWidget`
  (params (AbilityNeeded :type Integer))
  (returns (AbilityWidget :type "/Game/SkyesUIv2/Blueprints/UI/Widgets/W_Abilities Object Reference"))
  (bind _abilityuiwidgets (`self.AbilityUIWidgets`))
  (switch `int` (- AbilityNeeded 1)
    (:`0`
      (return (`|GetArrayItem` _abilityuiwidgets)))
    (:`1`
      (return (`|GetArrayItem` _abilityuiwidgets 1)))
    (:`2`
      (return (`|GetArrayItem` _abilityuiwidgets 2)))
    (:`3`
      (return (`|GetArrayItem` _abilityuiwidgets 3)))))

(fn `GetUltimateImage`
  (params (Ultimate :type "/Game/Rowan/E_Ultimate Enum" :default "NewEnumerator3"))
  (returns (`Ultimate Image` :type "Texture2D Object Reference"))
  (return (`BlueprintMapLibrary.Map_Find` (`self.Ultimate Image Map`) Ultimate)))

(fn `Map Range Clamped To Progress Bar`
  (params (`Current Value` :type "Float (double-precision)") (MinValue :type "Float (double-precision)") (MaxValue :type "Float (double-precision)"))
  (returns (ProgressBarValue :type "Float (double-precision)"))
  (return (`KismetMathLibrary.MapRangeClamped` `Current Value` MinValue MaxValue 0.0 1.0)))

(fn `SpawnNotifications`
  (params (Text :type Text) (TimeToRemainOnScreen :type "Float (double-precision)"))
  (returns (Notification :type "/Game/SkyesUIv2/Blueprints/UI/Widgets/W_NotificationsAlert Object Reference"))
  (bind _returnvalue (`|CreateWidget` "/Game/SkyesUIv2/Blueprints/UI/Widgets/W_NotificationsAlert.W_NotificationsAlert_C" null self TimeToRemainOnScreen))
  (`PanelWidget.AddChild` (`/Game/SkyesUIv2/Blueprints/UI/InGameUI.NotificationsBox` (`self.InGameUI`)) _returnvalue)
  (`TextBlock.SetText` (`/Game/SkyesUIv2/Blueprints/UI/Widgets/W_NotificationsAlert.NotificationText` _returnvalue) Text)
  (return _returnvalue))

(fn `UserConstructionScript`)