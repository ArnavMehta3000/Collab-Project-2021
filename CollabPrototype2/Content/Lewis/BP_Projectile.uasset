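; BP_Projectile is a damaging projectile that turns to face its Target actor when spawned.
; On hit or overlap, it sends damage and instigator through IHitMessage to the Target or any actor not exactly of class Bp_Enemy.
; It destroys itself only if that call returns true.
; I_GetProjectileMovement exposes its movement component and reports it as reflectable, while the other interface getters are empty.
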(event `self.ReceiveBeginPlay`
  (`self.K2_SetActorRotation` (`KismetMathLibrary.FindLookAtRotation` (`self.K2_GetActorLocation`) (`self.K2_GetActorLocation` (`self.Target`)))))

(event `self.ReceiveHit`
  (params (MyComp :type "PrimitiveComponent Object Reference") (Other :type "Actor Object Reference") (OtherComp :type "PrimitiveComponent Object Reference") (bSelfMoved :type Boolean) (HitLocation :type "Vector Structure") (HitNormal :type "Vector Structure") (NormalImpulse :type "Vector Structure") (Hit :type "HitResult Structure (by ref)"))
  (if (== Other (`self.Target`))
    (bind _succsess (message `/Game/Rowan/I_Hit.I_Hit` Other (`self.Instigator2`) (`self.Damage`) :!label _label))
    (if _succsess
      (`self.K2_DestroyActor`))
    (elif (not (== (`GameplayStatics.GetObjectClass` Other) "/Game/Lewis/Bp_Enemy.Bp_Enemy_C"))
      (goto _label))))

(event `self.ReceiveActorBeginOverlap`
  (params (OtherActor :type "Actor Object Reference"))
  (if (== OtherActor (`self.Target`))
    (bind _succsess (message `/Game/Rowan/I_Hit.I_Hit` OtherActor (`self.Instigator2`) (`self.Damage`) :!label _label_2))
    (if _succsess
      (`self.K2_DestroyActor`))
    (elif (not (== (`GameplayStatics.GetObjectClass` OtherActor) "/Game/Lewis/Bp_Enemy.Bp_Enemy_C"))
      (goto _label_2))))

(fn `I_Get Player Character`
  (returns (NewParam :type "/Game/Rowan/FirstPersonCharacterROwan Object Reference"))
  (return null))

(fn `I_GetGameMode`
  (returns (GetGameMode :type "/Game/Skye/FirstPersonTemplateBlueprints(TheseHaveBeenEdits)/FirstPersonGameModeSKYE Object Reference"))
  (return null))

(fn `I_GetPortaTurret`
  (returns (`Porta Turret` :type "/Game/Rowan/Porta_turret Object Reference"))
  (return null))

(fn `I_GetProjectileMovement`
  (returns (NewParam :type "ProjectileMovementComponent Object Reference") (Reflect :type Boolean))
  (return (`self.ProjectileMovement`) true))

(fn `UserConstructionScript`)