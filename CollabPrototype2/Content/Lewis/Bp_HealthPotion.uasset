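; Health potion pickup actor that restores a fixed amount of the player's health.
; On FirePickup, it calls IGetPlayerCharacter on FirstPersonChar and checks PlayerHealth against a threshold.
; Below that threshold it adds the health, prints the new value and destroys itself; otherwise the potion stays in the world.
; The construction script only calls its parent.
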(event `self.FirePickup`
  (bind _playerhealth (`self.PlayerHealth`))
  (`/Game/FirstPersonBP/Rowan/I_Cast.I_Get Player Character` (`self.FirstPersonChar`))
  (if (not (>= _playerhealth 75))
    (bind _output_get (set `/Game/Lewis/Bp_HealthPotion.PlayerHealth` (+ _playerhealth 25) null))
    (`KismetSystemLibrary.PrintString` (`KismetStringLibrary.Conv_IntToString` _output_get))
    (`self.K2_DestroyActor`)))

(fn `UserConstructionScript`
  (`parent.UserConstructionScript`))