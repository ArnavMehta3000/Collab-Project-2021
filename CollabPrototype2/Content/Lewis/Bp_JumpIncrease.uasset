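; Jump-increase pickup that boosts the player character's jump when its FirePickup event runs.
; FirePickup gets the player through an interface message on a FirstPersonChar reference, calls IncreaseJump on it, then destroys the pickup.
; The other interface getters are empty stubs, and the projectile movement getter returns Reflect as false.
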(event `self.FirePickup`
  (bind _newparam (message `/Game/Rowan/I_Cast.I_Get Player Character` (`self.FirstPersonChar`)))
  (`/Game/Rowan/FirstPersonCharacterROwan.IncreaseJump` _newparam)
  (`self.K2_DestroyActor`))

(fn `I_Get Game Instance`
  (returns (`Game Instance` :type "/Game/Rowan/Cyber_Instance Object Reference"))
  (return null))

(fn `I_Get Lobby Gamemode`
  (returns (Gamemode :type "/Game/Rowan/Lobby_Gamemode Object Reference"))
  (return null))

(fn `I_Get Player Character`
  (returns (NewParam :type "/Game/Rowan/FirstPersonCharacterROwan Object Reference"))
  (return null))

(fn `I_Get World UI`
  (returns (`CHeck Box` :type "/Game/Rowan/CHeckBox2 Object Reference") (`Shop Node` :type "/Game/Rowan/Shop_Node Object Reference"))
  (return null null))

(fn `I_GetGameMode`
  (returns (GetGameMode :type "/Game/PrimaryGameMode Object Reference"))
  (return null))

(fn `I_GetPortaTurret`
  (returns (`Porta Turret` :type "/Game/Rowan/Porta_turret Object Reference"))
  (return null))

(fn `I_GetProjectileMovement`
  (returns (NewParam :type "ProjectileMovementComponent Object Reference") (Reflect :type Boolean))
  (return null false))

(fn `UserConstructionScript`
  (`parent.UserConstructionScript`))