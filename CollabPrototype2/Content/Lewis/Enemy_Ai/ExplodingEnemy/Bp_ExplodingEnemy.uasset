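; Exploding enemy character that self-destructs when the player enters its trigger sphere.
; After a two-second delay it fires a radial impulse, spawns an emitter, deals radial damage and destroys itself.
; Hits reduce HP through an interface; death by damage credits the instigating player and may drop a random pickup.
; Both deaths notify the room manager, which is supplied through an interface event.
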(event `self.Sphere.OnComponentBeginOverlap`
  (params (OverlappedComponent :type "PrimitiveComponent Object Reference") (OtherActor :type "Actor Object Reference") (OtherComp :type "PrimitiveComponent Object Reference") (OtherBodyIndex :type Integer) (bFromSweep :type Boolean) (SweepResult :type "HitResult Structure (by ref)"))
  (bind _returnvalue (`self.K2_GetActorLocation`))
  (bind _asfirst_person_character_rowan (cast `/Game/Rowan/FirstPersonCharacterROwan` OtherActor))
  (if (== _asfirst_person_character_rowan OtherActor)
    (`KismetSystemLibrary.Delay` 2.0)
    (`RadialForceComponent.FireImpulse` (`self.Explosion`))
    (`GameplayStatics.SpawnEmitterAtLocation` null _returnvalue (struct) (2.0 2.0 2.0))
    (`GameplayStatics.ApplyRadialDamage` :`BaseDamage` 30.0 :`Origin` _returnvalue :`DamageRadius` 800.0 :`DamageCauser` null :`InstigatedByController` null)
    (`/Game/Rowan/Room_Manager_Integrated.Enemy Downed` (`self.Manager`))
    (`self.K2_DestroyActor`)))

(event `/Game/Rowan/I_Cast.I_GetRoomManager`
  (params (Manager :type "/Game/Rowan/Room_Manager_Integrated Object Reference"))
  (set `self.Manager` Manager))

(fn `I_Get Player Character`
  (returns (NewParam :type "/Game/Rowan/FirstPersonCharacterROwan Object Reference"))
  (return null))

(fn `I_GetGameMode`
  (returns (GetGameMode :type "/Game/Skye/FirstPersonTemplateBlueprints(TheseHaveBeenEdits)/FirstPersonGameModeSKYE Object Reference"))
  (return null))

(fn `I_GetPortaTurret`
  (returns (`Porta Turret` :type "/Game/Rowan/Porta_turret Object Reference"))
  (return null))

(fn `I_GetProjectileMovement`
  (returns (NewParam :type "ProjectileMovementComponent Object Reference") (Reflect :type Boolean))
  (return null false))

(fn `I_Hit`
  (params (Instiagator :type "Actor Object Reference (by ref)") (Damage :type "Float (double-precision)"))
  (returns (Succsess :type Boolean))
  (bind _output_get (set `self.HP` (- (`self.HP`) Damage)))
  (if (<= _output_get 0.0)
    (bind _newparam (message `/Game/Rowan/I_Cast.I_Get Player Character` Instiagator))
    (if (`KismetSystemLibrary.IsValid` _newparam)
      (`/Game/Rowan/FirstPersonCharacterROwan.Enemy Kill` _newparam))
    (`self.RandomDrop`)
    (`/Game/Rowan/Room_Manager_Integrated.Enemy Downed` (`self.Manager`))
    (`self.K2_DestroyActor`)
    (return true)))

(fn `RandomDrop`
  (bind _pickups (`self.Pickups`))
  (if (== 0 (`KismetMathLibrary.RandomIntegerInRange` 0 3))
    (`|SpawnActorFromClass` (`|GetArrayItem` _pickups (`KismetMathLibrary.RandomIntegerInRange` 0 (`KismetArrayLibrary.Array_Length` _pickups))) (`self.GetTransform`) "Undefined" "OverrideRootScale" null null)))

(fn `UpdateMoveSpeed`
  (params (MaxWalkSpeed :type "Float (double-precision)"))
  (set `CharacterMovementComponent.MaxWalkSpeed` MaxWalkSpeed (`self.CharacterMovement`)))

(fn `UserConstructionScript`)