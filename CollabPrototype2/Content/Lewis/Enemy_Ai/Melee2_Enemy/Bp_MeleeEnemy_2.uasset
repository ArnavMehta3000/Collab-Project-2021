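; Melee enemy variant that attacks a target, takes damage and reports its death to the room manager.
; Attack plays a random slot animation and sends interface hit damage, rate-limited by a timer-reset DoOnce.
; Radial damage routes into the hit interface; death credits the player, may drop a pickup and destroys the actor.
; Healing clears its HealAI timer immediately after setting it, and the CT_Enemy spawn chain is disconnected.
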(event `self.ReceiveBeginPlay`
  (set `self.HP` 100.0))

(event `Attack`
  (params (Target :type "Actor Object Reference"))
  (`/Engine/EditorBlueprintResources/StandardMacros.DoOnce` false :!label _label
    (:`Completed`
      (`AnimInstance.PlaySlotAnimation` (`SkeletalMeshComponent.GetAnimInstance` (`self.Mesh`)) (select `bool` (`KismetMathLibrary.RandomBool`) :`false` "/Game/EnemyMeshes/Oni/Animations/OniAnimDoubleAttack.OniAnimDoubleAttack" :`true` "/Game/EnemyMeshes/Oni/Animations/OniAnimJab.OniAnimJab" :!type "AnimSequenceBase Object Reference") "Attack" 0.25 0.25 1.0 1)
      (message `/Game/Rowan/I_Hit.I_Hit` Target self (`self.Damage`))
      (`KismetSystemLibrary.K2_SetTimerDelegate` (delegate `Reset`) (`self.Attack Rate`)))))

(event `Reset`
  (goto _label :!via `Reset`))

(event `/Game/Rowan/I_Cast.I_GetRoomManager`
  (params (Manager :type "/Game/Rowan/Room_Manager_Integrated Object Reference"))
  (set `self.Manager` Manager))

(event `self.ReceiveRadialDamage`
  (params (DamageReceived :type "Float (single-precision)") (DamageType :type "DamageType Object Reference") (Origin :type "Vector Structure") (HitInfo :type "HitResult Structure (by ref)") (InstigatedBy :type "Controller Object Reference") (DamageCauser :type "Actor Object Reference"))
  (message `/Game/Rowan/I_Hit.I_Hit` self InstigatedBy DamageReceived))

(event `/Game/Lewis/Interfaces/i_Heal.I_Heal`
  (if (not (== (`self.HP`) 200.0))
    (bind _returnvalue (`KismetSystemLibrary.K2_SetTimerDelegate` (delegate `Heal AI`) 0.0 (`self.Looping`)))
    (`KismetSystemLibrary.K2_ClearAndInvalidateTimerHandle` _returnvalue)
    (set `self.HealthTimer` 20)
    (`KismetSystemLibrary.Delay` 7.0)
    (set `self.Looping` true)))

(event `Heal AI`
  (bind _healthtimer (`self.HealthTimer`))
  (`/Engine/EditorBlueprintResources/StandardMacros.IncrementFloat` (`self.HP`)
    (:`  `
      (`/Engine/EditorBlueprintResources/StandardMacros.DecrementInt` _healthtimer
        (:`  `
          (if (== _healthtimer 0)
            (set `self.Looping` false)
            (else
              (`KismetSystemLibrary.PrintString` "Healing"))))))))

(fn `I_Get Game Instance`
  (returns (`Game Instance` :type "/Game/Rowan/Cyber_Instance Object Reference"))
  (return null))

(fn `I_Get Lobby Gamemode`
  (returns (Gamemode :type "/Game/Rowan/Lobby_Gamemode Object Reference"))
  (return null))

(fn `I_Get Player Character`
  (returns (NewParam :type "/Game/Rowan/FirstPersonCharacterROwan Object Reference"))
  (return null))

(fn `I_Get World UI`
  (returns (`CHeck Box` :type "/Game/Rowan/CHeckBox2 Object Reference") (`Shop Node` :type "/Game/Rowan/Shop_Node Object Reference"))
  (return null null))

(fn `I_GetGameMode`
  (returns (GetGameMode :type "/Game/PrimaryGameMode Object Reference"))
  (return null))

(fn `I_GetPortaTurret`
  (returns (`Porta Turret` :type "/Game/Rowan/Porta_turret Object Reference"))
  (return null))

(fn `I_GetProjectileMovement`
  (returns (NewParam :type "ProjectileMovementComponent Object Reference") (Reflect :type Boolean))
  (return null false))

(fn `I_Hit`
  (params (Instiagator :type "Actor Object Reference (by ref)") (Damage :type "Float (double-precision)"))
  (returns (Succsess :type Boolean))
  (bind _output_get (set `self.HP` (- (`self.HP`) Damage)))
  (if (<= _output_get 0.0)
    (bind _newparam (message `/Game/Rowan/I_Cast.I_Get Player Character` Instiagator))
    (if (`KismetSystemLibrary.IsValid` _newparam)
      (`/Game/Rowan/FirstPersonCharacterROwan.Enemy Kill` _newparam 0))
    (`self.Random Drop`)
    (`/Game/Rowan/Room_Manager_Integrated.Enemy Downed` (`self.Manager`))
    (`self.K2_DestroyActor`)
    (return false)))

(fn `Random Drop`
  (bind _pickups (`self.Pickups`))
  (if (== 0 (`KismetMathLibrary.RandomIntegerInRange` 0 3))
    (`|SpawnActorFromClass` (`|GetArrayItem` _pickups (`KismetMathLibrary.RandomIntegerInRange` 0 (`KismetArrayLibrary.Array_Length` _pickups))) (`self.GetTransform`) "Undefined" "OverrideRootScale" null null)))

(fn `UserConstructionScript`)