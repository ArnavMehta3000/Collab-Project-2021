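; Healing enemy that supports other enemies, with scaled max HP, a player-facing health bar and kill handling.
; HealAlly scans "Enemy"-tagged actors for nearer ones, turns toward them and, if damaged, heals them through interface messages with an animation and a temporary cable link.
; On lethal hits it credits the instigating player's score, usually drops a random pickup, notifies its room manager and destroys itself.
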(event `Heal Ally`
  (bind _nearest_actor (`self.Nearest Actor`))
  (bind _healthcable (`self.HealthCable`))
  (bind (_returnvalue_roll _returnvalue_pitch _returnvalue_yaw) (`KismetMathLibrary.BreakRotator` (`KismetMathLibrary.RInterpTo` (`self.K2_GetActorRotation`) (`KismetMathLibrary.FindLookAtRotation` (`self.K2_GetActorLocation`) (`self.K2_GetActorLocation` (`self.Nearest Actor`))) (`GameplayStatics.GetWorldDeltaSeconds`))))
  ;[1 1 1] Finds closest pawn and then rotates to face it.
  (if (`self.Condition`)
    (bind _outactors (`GameplayStatics.GetAllActorsWithTag` "Enemy"))
    (for _array_element _outactors
      (bind _returnvalue (`KismetMathLibrary.Vector_Distance` (`self.K2_GetActorLocation` _array_element) (`SceneComponent.K2_GetComponentLocation` (`self.CapsuleComponent`))))
      (if (< _returnvalue (`self.Nearest Distance`))
        (set `self.Nearest Distance` _returnvalue)
        (set `self.Nearest Actor` _array_element)
        (`self.K2_SetActorRotation` (`KismetMathLibrary.MakeRotator` 0.0 0.0 _returnvalue_yaw))
        ;[1 1 1] Detects Whether it hits an "Enemy" actor.
        (bind (_health _maxhealth) (message `/Game/Lewis/Interfaces/i_Heal.I_GetHealth` (`self.Nearest Actor`)))
        (if (!= _health _maxhealth)
          (`AnimInstance.PlaySlotAnimation` (`SkeletalMeshComponent.GetAnimInstance` (`self.Mesh`)) "/Game/EnemyMeshes/Kitsune/kitsuneheal.kitsuneheal" "Attack" 0.25 0.25 1.0 1)
          (message `/Game/Lewis/Interfaces/i_Heal.I_Heal` _nearest_actor)
          (`CableComponent.SetAttachEndTo` _healthcable _nearest_actor "None" "None")
          (`SceneComponent.SetVisibility` _healthcable true false)
          (`KismetSystemLibrary.K2_SetTimerDelegate` (delegate `Stop Heal`) 3.0))))))

(event `Stop Heal`
  ;[1 1 1] Detects Whether it hits an "Enemy" actor.
  (`SceneComponent.SetVisibility` (`self.HealthCable`) false false))

(event `/Game/Rowan/I_Cast.I_GetRoomManager`
  (params (Manager :type "/Game/Rowan/Room_Manager_Integrated Object Reference"))
  (set `self.Manager` Manager))

(event `self.ReceiveBeginPlay`
  (bind _asw_enemy_hp (cast `/Game/SkyesUIv2/Blueprints/UI/Widgets/W_EnemyHP` (`WidgetComponent.GetWidget` (`self.HPBar`)) :!pure true))
  (bind _getgamemode (message `/Game/Rowan/I_Cast.I_GetGameMode` (`GameplayStatics.GetGameMode`)))
  (set `self.MaxHP` (+ (`self.MaxHP`) (`KismetMathLibrary.Conv_IntToDouble` (* (`/Game/PrimaryGameMode.Enemy scale` _getgamemode) 10))))
  (set `self.HP` (`self.MaxHP`))
  ;[1 1 1] Setup HP Bar
  (`/Game/SkyesUIv2/Blueprints/UI/Widgets/W_EnemyHP.SetHPBar` _asw_enemy_hp (`self.HP`) (`self.MaxHP`))
  (set `self.EnemyHPBar` _asw_enemy_hp))

(event `self.ReceiveTick`
  (params (DeltaSeconds :type "Float (single-precision)"))
  ;[1 1 1] Face HP Bar to Player
  (bind _newparam (message `/Game/Rowan/I_Cast.I_Get Player Character` (`GameplayStatics.GetPlayerCharacter` 0)))
  (bind _returnvalue_location (`KismetMathLibrary.BreakTransform` (`SceneComponent.K2_GetComponentToWorld` (`Character.CapsuleComponent` _newparam))))
  (`self.WhereToFaceHPBar` _returnvalue_location))

(fn `I_Get Game Instance`
  (returns (`Game Instance` :type "/Game/Rowan/Cyber_Instance Object Reference"))
  (return null))

(fn `I_Get Lobby Gamemode`
  (returns (Gamemode :type "/Game/Rowan/Lobby_Gamemode Object Reference"))
  (return null))

(fn `I_Get Player Character`
  (returns (NewParam :type "/Game/Rowan/FirstPersonCharacterROwan Object Reference"))
  (return null))

(fn `I_Get World UI`
  (returns (`CHeck Box` :type "/Game/Rowan/CHeckBox2 Object Reference") (`Shop Node` :type "/Game/Rowan/Shop_Node Object Reference"))
  (return null null))

(fn `I_GetGameMode`
  (returns (GetGameMode :type "/Game/PrimaryGameMode Object Reference"))
  (return null))

(fn `I_GetPortaTurret`
  (returns (`Porta Turret` :type "/Game/Rowan/Porta_turret Object Reference"))
  (return null))

(fn `I_GetProjectileMovement`
  (returns (NewParam :type "ProjectileMovementComponent Object Reference") (Reflect :type Boolean))
  (return null false))

(fn `I_Hit`
  (params (Instiagator :type "Actor Object Reference (by ref)") (Damage :type "Float (double-precision)"))
  (returns (Succsess :type Boolean))
  (bind _output_get (set `self.HP` (- (`self.HP`) Damage)))
  ;[1 1 1] Update HP Bar
  (`/Game/SkyesUIv2/Blueprints/UI/Widgets/W_EnemyHP.SetHPBar` (`self.EnemyHPBar`) (`self.HP`) (`self.MaxHP`))
  (if (<= _output_get 0.0)
    (bind _newparam (message `/Game/Rowan/I_Cast.I_Get Player Character` Instiagator))
    (if (`KismetSystemLibrary.IsValid` _newparam)
      (`/Game/Rowan/FirstPersonCharacterROwan.Enemy Kill` _newparam (`self.Score`)))
    (`self.Random Drop`)
    (`/Game/Rowan/Room_Manager_Integrated.Enemy Downed` (`self.Manager`))
    (`self.K2_DestroyActor`)
    (return false)))

(fn `Random Drop`
  (bind _pickups (`self.Pickups`))
  (if (!= (`KismetMathLibrary.RandomIntegerInRange` 0 5) 0)
    (`|SpawnActorFromClass` (`|GetArrayItem` _pickups (`KismetMathLibrary.RandomIntegerInRange` 0 (`KismetArrayLibrary.Array_Length` _pickups))) (`self.GetTransform`) "Undefined" "OverrideRootScale" null null)))

(fn `UserConstructionScript`)

(fn `WhereToFaceHPBar`
  (params (InputPin :type "Vector Structure (by ref)"))
  (bind _hpbar (`self.HPBar`))
  (`SceneComponent.K2_SetWorldRotation` _hpbar (`KismetMathLibrary.FindLookAtRotation` (`SceneComponent.K2_GetComponentLocation` _hpbar) InputPin) false false))