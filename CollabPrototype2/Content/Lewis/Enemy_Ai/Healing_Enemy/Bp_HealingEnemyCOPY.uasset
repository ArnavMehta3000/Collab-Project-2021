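; Healing enemy that restores nearby damaged allies, takes hits and can drop a pickup on death.
; HealAlly scans "Enemy"-tagged actors, turns toward any closer than the stored nearest distance and heals it through interface messages if below max health, showing an attached cable until a timer hides it.
; IHit subtracts damage and, at zero HP, credits the instigator's kill, rolls a random drop, notifies the manager and destroys the actor.
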(event `Heal Ally`
  (bind _healthcable (`self.HealthCable`))
  (bind _nearest_actor (`self.Nearest Actor`))
  (bind (_returnvalue_roll _returnvalue_pitch _returnvalue_yaw) (`KismetMathLibrary.BreakRotator` (`KismetMathLibrary.RInterpTo` (`self.K2_GetActorRotation`) (`KismetMathLibrary.FindLookAtRotation` (`self.K2_GetActorLocation`) (`self.K2_GetActorLocation` (`self.Nearest Actor`))) (`GameplayStatics.GetWorldDeltaSeconds`))))
  ;[1 1 1] Finds closest pawn and then rotates to face it.
  (if (`self.Condition`)
    (bind _outactors (`GameplayStatics.GetAllActorsWithTag` "Enemy"))
    (for _array_element _outactors
      (bind _returnvalue (`KismetMathLibrary.Vector_Distance` (`self.K2_GetActorLocation` _array_element) (`SceneComponent.K2_GetComponentLocation` (`self.CapsuleComponent`))))
      (if (< _returnvalue (`self.Nearest Distance`))
        (set `self.Nearest Distance` _returnvalue)
        (set `self.Nearest Actor` _array_element)
        (`self.K2_SetActorRotation` (`KismetMathLibrary.MakeRotator` 0.0 0.0 _returnvalue_yaw))
        ;[1 1 1] Detects Whether it hits an "Enemy" actor.
        (bind (_health _maxhealth) (message `/Game/Lewis/Interfaces/i_Heal.I_GetHealth` (`self.Nearest Actor`)))
        (if (!= _health _maxhealth)
          (message `/Game/Lewis/Interfaces/i_Heal.I_Heal` _nearest_actor)
          (`CableComponent.SetAttachEndTo` _healthcable _nearest_actor "None" "None")
          (`SceneComponent.SetVisibility` _healthcable true false)
          (`KismetSystemLibrary.K2_SetTimerDelegate` (delegate `Stop Heal`) 3.0))))))

(event `Stop Heal`
  ;[1 1 1] Detects Whether it hits an "Enemy" actor.
  (`SceneComponent.SetVisibility` (`self.HealthCable`) false false))

(fn `I_Hit`
  (params (Instiagator :type "Actor Object Reference (by ref)") (Damage :type "Float (double-precision)"))
  (returns (Succsess :type Boolean))
  (bind _output_get (set `self.HP` (- (`self.HP`) Damage)))
  (if (<= _output_get 0.0)
    (bind _newparam (message `/Game/Rowan/I_Cast.I_Get Player Character` Instiagator))
    (if (`KismetSystemLibrary.IsValid` _newparam)
      (`/Game/Rowan/FirstPersonCharacterROwan.Enemy Kill` _newparam))
    (`self.Random Drop`)
    (`/Game/Rowan/Room_Manager_Integrated.Enemy Downed` (`self.Manager`))
    (`self.K2_DestroyActor`)
    (return false)))

(fn `Random Drop`
  (bind _pickups (`self.Pickups`))
  (if (== 0 (`KismetMathLibrary.RandomIntegerInRange` 0 3))
    (`|SpawnActorFromClass` (`|GetArrayItem` _pickups (`KismetMathLibrary.RandomIntegerInRange` 0 (`KismetArrayLibrary.Array_Length` _pickups))) (`self.GetTransform`) "Undefined" "OverrideRootScale" null null)))

(fn `UserConstructionScript`)