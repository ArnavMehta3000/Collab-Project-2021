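; Double melee enemy Blueprint that attacks targets, takes damage and can be healed, using interface messages.
; Attacks pass through a DoOnce that a timer resets at the attack rate, and radial damage routes into the hit interface.
; Healing runs a looping timer that adds HP over a fixed number of ticks.
; On death it credits the killer, randomly drops a pickup, notifies its room manager and destroys itself.
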(event `self.ReceiveBeginPlay`
  (set `self.HP` (`self.MaxHealth`)))

(event `Attack`
  (params (Target :type "Actor Object Reference"))
  (`/Engine/EditorBlueprintResources/StandardMacros.DoOnce` false :!label _label
    (:`Completed`
      (message `/Game/Rowan/I_Hit.I_Hit` Target self (`self.Damage`))
      (`KismetSystemLibrary.K2_SetTimerDelegate` (delegate `Reset`) (`self.Attack Rate`)))))

(event `Reset`
  (goto _label :!via `Reset`))

(event `/Game/Rowan/I_Cast.I_GetRoomManager`
  (params (Manager :type "/Game/Rowan/Room_Manager_Integrated Object Reference"))
  (set `self.Manager` Manager))

(event `self.ReceiveRadialDamage`
  (params (DamageReceived :type "Float (single-precision)") (DamageType :type "DamageType Object Reference") (Origin :type "Vector Structure") (HitInfo :type "HitResult Structure (by ref)") (InstigatedBy :type "Controller Object Reference") (DamageCauser :type "Actor Object Reference"))
  (message `/Game/Rowan/I_Hit.I_Hit` self InstigatedBy DamageReceived))

(event `/Game/Lewis/Interfaces/i_Heal.I_Heal`
  (if (not (== (`self.HP`) (`self.MaxHealth`)))
    (bind _returnvalue (`KismetSystemLibrary.K2_SetTimerDelegate` (delegate `Heal AI`) 0.2 true))
    (set `self.Timer` _returnvalue)
    (set `self.HealthTimer` 20)
    (`/Engine/EditorBlueprintResources/StandardMacros.IncrementFloat` (`self.HP`) :!label _label_2
      (:`  `
        (bind _result (`/Engine/EditorBlueprintResources/StandardMacros.DecrementInt` (`self.HealthTimer`))
          (:`  `
            (if (== _result 0)
              (`KismetSystemLibrary.K2_ClearAndInvalidateTimerHandle` (`self.Timer`))
              (`KismetSystemLibrary.PrintString` (`KismetStringLibrary.Conv_DoubleToString` (`self.HP`)))
              (else
                (`KismetSystemLibrary.PrintString` "Healing")))))))))

(event `Heal AI`
  (goto _label_2))

(fn `I_Get Player Character`
  (returns (NewParam :type "/Game/Rowan/FirstPersonCharacterROwan Object Reference"))
  (return null))

(fn `I_GetGameMode`
  (returns (GetGameMode :type "/Game/Skye/FirstPersonTemplateBlueprints(TheseHaveBeenEdits)/FirstPersonGameModeSKYE Object Reference"))
  (return null))

(fn `I_GetHealth`
  (returns (Health :type "Float (double-precision)") (MaxHealth :type "Float (double-precision)"))
  (return (`self.HP`) (`self.MaxHealth`)))

(fn `I_GetPortaTurret`
  (returns (`Porta Turret` :type "/Game/Rowan/Porta_turret Object Reference"))
  (return null))

(fn `I_GetProjectileMovement`
  (returns (NewParam :type "ProjectileMovementComponent Object Reference") (Reflect :type Boolean))
  (return null false))

(fn `I_Hit`
  (params (Instiagator :type "Actor Object Reference (by ref)") (Damage :type "Float (double-precision)"))
  (returns (Succsess :type Boolean))
  (bind _output_get (set `self.HP` (- (`self.HP`) Damage)))
  (if (<= _output_get 0.0)
    (bind _newparam (message `/Game/Rowan/I_Cast.I_Get Player Character` Instiagator))
    (if (`KismetSystemLibrary.IsValid` _newparam)
      (`/Game/Rowan/FirstPersonCharacterROwan.Enemy Kill` _newparam))
    (`self.Random Drop`)
    (`/Game/Rowan/Room_Manager_Integrated.Enemy Downed` (`self.Manager`))
    (`self.K2_DestroyActor`)
    (return false)))

(fn `Random Drop`
  (bind _pickups (`self.Pickups`))
  (if (== 0 (`KismetMathLibrary.RandomIntegerInRange` 0 3))
    (`|SpawnActorFromClass` (`|GetArrayItem` _pickups (`KismetMathLibrary.RandomIntegerInRange` 0 (`KismetArrayLibrary.Array_Length` _pickups))) (`self.GetTransform`) "Undefined" "OverrideRootScale" null null)))

(fn `UserConstructionScript`)