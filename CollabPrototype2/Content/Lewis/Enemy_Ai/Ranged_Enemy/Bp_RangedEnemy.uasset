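; Ranged AI enemy character that shoots bullets at a target and reports its death to a room manager.
; Fire plays an attack animation and spawns an aimed BP_Bullet, using a DoOnce that a timer resets as a cooldown.
; Tick feeds HP to its BasicCrowdController's Below25 check, while IHeal drives timer-based healing.
; Radial damage routes into the hit interface; death awards player score, may drop a random pickup and destroys the actor.
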(event `self.ReceiveBeginPlay`
  (set `self.HP` (`self.MaxHP`)))

(event `self.ReceiveTick`
  (params (DeltaSeconds :type "Float (single-precision)"))
  (`/Game/Lewis/Enemy_Ai/Ranged_Enemy/BasicCrowdController.Below 25%` (cast `/Game/Lewis/Enemy_Ai/Ranged_Enemy/BasicCrowdController` (`self.GetController`) :!pure true) (`self.HP`)))

(event `Fire`
  (params (Target :type "Actor Object Reference"))
  (bind _returnvalue (`SceneComponent.K2_GetComponentLocation` (`self.Sphere1`)))
  (`/Engine/EditorBlueprintResources/StandardMacros.DoOnce` false :!label _label
    (:`Completed`
      (`AnimInstance.PlaySlotAnimation` (`SkeletalMeshComponent.GetAnimInstance` (`self.Mesh`)) "/Game/EnemyMeshes/Yuuki-ona/yuki-onna_action.yuki-onna_action" "Attack" 0.25 0.25 1.0 1)
      (bind _returnvalue_2 (`|SpawnActorFromClass` "/Game/Arnav/Shooting/BP_Bullet.BP_Bullet_C" (`KismetMathLibrary.MakeTransform` _returnvalue (`KismetMathLibrary.FindLookAtRotation` _returnvalue (`self.K2_GetActorLocation` Target))) "AdjustIfPossibleButAlwaysSpawn" "OverrideRootScale" null null))
      (`/Engine/EditorBlueprintResources/StandardMacros.IsValid` _returnvalue_2
        (:`Is Valid`
          (`/Game/Arnav/Shooting/BP_Bullet.InitializeBullet` _returnvalue_2 null 1000.0 10.0 0)
          (`KismetSystemLibrary.K2_SetTimerDelegate` (delegate `SpawnProjectile`) 1.0))))))

(event `SpawnProjectile`
  (goto _label :!via `Reset`))

(event `/Game/Rowan/I_Cast.I_GetRoomManager`
  (params (Manager :type "/Game/Rowan/Room_Manager_Integrated Object Reference"))
  (set `self.Manager` Manager))

(event `self.ReceiveRadialDamage`
  (params (DamageReceived :type "Float (single-precision)") (DamageType :type "DamageType Object Reference") (Origin :type "Vector Structure") (HitInfo :type "HitResult Structure (by ref)") (InstigatedBy :type "Controller Object Reference") (DamageCauser :type "Actor Object Reference"))
  (message `/Game/Rowan/I_Hit.I_Hit` self InstigatedBy DamageReceived))

(event `/Game/Lewis/Interfaces/i_Heal.I_Heal`
  (if (not (== (`self.HP`) (`self.MaxHP`)))
    (bind _returnvalue (`KismetSystemLibrary.K2_SetTimerDelegate` (delegate `Heal AI`) 0.0 (`self.Looping`)))
    (`KismetSystemLibrary.K2_ClearAndInvalidateTimerHandle` _returnvalue)
    (set `self.HealthTimer` 20)
    (`KismetSystemLibrary.Delay` 7.0)
    (set `self.Looping` true)))

(event `Heal AI`
  (bind _healthtimer (`self.HealthTimer`))
  (`/Engine/EditorBlueprintResources/StandardMacros.IncrementFloat` (`self.HP`)
    (:`  `
      (`/Engine/EditorBlueprintResources/StandardMacros.DecrementInt` _healthtimer
        (:`  `
          (if (== _healthtimer 0)
            (set `self.Looping` false)
            (else
              (`KismetSystemLibrary.PrintString` "Healing"))))))))

(fn `I_Get Game Instance`
  (returns (`Game Instance` :type "/Game/Rowan/Cyber_Instance Object Reference"))
  (return null))

(fn `I_Get Lobby Gamemode`
  (returns (Gamemode :type "/Game/Rowan/Lobby_Gamemode Object Reference"))
  (return null))

(fn `I_Get Player Character`
  (returns (NewParam :type "/Game/Rowan/FirstPersonCharacterROwan Object Reference"))
  (return null))

(fn `I_Get World UI`
  (returns (`CHeck Box` :type "/Game/Rowan/CHeckBox2 Object Reference") (`Shop Node` :type "/Game/Rowan/Shop_Node Object Reference"))
  (return null null))

(fn `I_GetGameMode`
  (returns (GetGameMode :type "/Game/PrimaryGameMode Object Reference"))
  (return null))

(fn `I_GetHealth`
  (returns (Health :type "Float (double-precision)") (MaxHealth :type "Float (double-precision)"))
  (return (`self.HP`) (`self.MaxHP`)))

(fn `I_GetPortaTurret`
  (returns (`Porta Turret` :type "/Game/Rowan/Porta_turret Object Reference"))
  (return null))

(fn `I_GetProjectileMovement`
  (returns (NewParam :type "ProjectileMovementComponent Object Reference") (Reflect :type Boolean))
  (return null false))

(fn `I_Hit`
  (params (Instiagator :type "Actor Object Reference (by ref)") (Damage :type "Float (double-precision)"))
  (returns (Succsess :type Boolean))
  (bind _output_get (set `self.HP` (- (`self.HP`) Damage)))
  (if (<= _output_get 0.0)
    (bind _newparam (message `/Game/Rowan/I_Cast.I_Get Player Character` Instiagator))
    (if (`KismetSystemLibrary.IsValid` _newparam)
      (`/Game/Rowan/FirstPersonCharacterROwan.Enemy Kill` _newparam (`self.Score`)))
    (`self.RandomDrop`)
    (`/Game/Rowan/Room_Manager_Integrated.Enemy Downed` (`self.Manager`))
    (`self.K2_DestroyActor`)
    (return true)))

(fn `RandomDrop`
  (bind _pickups (`self.Pickups`))
  (if (== 0 (`KismetMathLibrary.RandomIntegerInRange` 0 3))
    (`|SpawnActorFromClass` (`|GetArrayItem` _pickups (`KismetMathLibrary.RandomIntegerInRange` 0 (`KismetArrayLibrary.Array_Length` _pickups))) (`self.GetTransform`) "Undefined" "OverrideRootScale" null null)))

(fn `UpdateMoveSpeed`
  (params (MaxWalkSpeed :type "Float (double-precision)"))
  (set `CharacterMovementComponent.MaxWalkSpeed` MaxWalkSpeed (`self.CharacterMovement`)))

(fn `UserConstructionScript`)